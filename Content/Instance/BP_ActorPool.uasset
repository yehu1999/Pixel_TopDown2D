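; BP_ActorPool is the central object pool for monsters, character and monster projectiles, summons, items and objects.
; Awake functions reuse a sleeping actor or spawn one, then teleport it; character projectiles and summons are capped.
; BeginPlay initializes DataTable data assets, then spawns and possesses the character once the pool reference is valid.
; Game mode starts delayed, staggered off-screen monster waking to avoid re-picking waking actors; Tick refills monsters and prints pool counts.
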(event `Apply_GameMode`
  (params (E_Mode :type "/Game/BluePrints/Modes/E_Mode Enum" :default "NewEnumerator0"))
  (switch `/Game/BluePrints/Modes/E_Mode` E_Mode
    (:`NewEnumerator0`
      _)
    (:`NewEnumerator1`
      _))
  ;[1 1 1] MonsterInvade
  (`KismetSystemLibrary.Delay` 1.0)
  (`self.Awake_Num_Monster` (`self.Max_Monster_Num`)))

(event `self.ReceiveBeginPlay`
  (`self.Init_DataAssets`)
  (`/Engine/EditorBlueprintResources/StandardMacros.IsValid` (`/Game/Instance/Public/FL_Public.Get_ActorPool`) :!label _label
    (:`Is Valid`
      (`self.Spawn Character`))
    (:`Is Not Valid`
      (`KismetSystemLibrary.DelayUntilNextTick`) ; 等待游戏实例将ActorPool保存为变量\n否则Character初始化中的\nGetActorPool将无效获取
      (goto _label))))

(event `self.ReceiveTick`
  (params (DeltaSeconds :type "Float (single-precision)"))
  (`self.DEBUG_Print_PoolNum`)
  (`self.TryTo_Fillup_MonsterPool`))

(event `Awake_Num_Monster`
  (params (Num :type Integer))
  ;[1 1 1] Monster
  (set `self.MonsterLoop_Num` Num)
  (`self.Loop_Awake_Monster`))

(event `Loop_Awake_Monster`
  ;[1 1 1] Monster
  (`KismetSystemLibrary.Delay` 0.2)
  (bind _random_outviewport_spawnlocation (`self.Get Random Out Viewport Spawn Location`))
  (bind _outrownames (`DataTableFunctionLibrary.GetDataTableRowNames` "/Game/BluePrints/Entities/Monsters/DT_Monster.DT_Monster"))
  (`self.Awake_A_Monster` (`KismetArrayLibrary.Array_Random` _outrownames) _random_outviewport_spawnlocation)
  (if (>= (`self.MonsterLoop_Index`) (`self.MonsterLoop_Num`))
    (set `self.MonsterLoop_Index` 1)
    (else
      (`/Engine/EditorBlueprintResources/StandardMacros.IncrementInt` (`self.MonsterLoop_Index`)
        (:`  `
          (`self.Loop_Awake_Monster`))))))

(fn `Awake_A_Item`
  (params (Item_RowName :type Name) (DestLocation :type "Vector Structure"))
  (locals (Local_Accessible_Item :type "/Game/BluePrints/Objects/Item/BP_Item Object Reference"))
  (bind _local_accessible_item (`local.Local_Accessible_Item`))
  (for _array_element (`self.ItemPool`)
    (if (`|EnumEquality` (`/Game/BluePrints/Objects/Item/BP_Item.Item_State` _array_element) "NewEnumerator1")
      (set `local.Local_Accessible_Item` _array_element)
      (break)))
  (`local.Local_Accessible_Item`
    (:`then`
      _)
    (:`else`
      (bind _returnvalue (`|SpawnActorFromClass` "/Game/BluePrints/Objects/Item/BP_Item.BP_Item_C" (`KismetMathLibrary.MakeTransform` (0.0 0.0 50000.0)) "Undefined" "MultiplyWithRoot" null Item_RowName null)) ; 没有可用对象则生成对象
      (bind _output_get (set `local.Local_Accessible_Item` _returnvalue))
      (`KismetArrayLibrary.Array_AddUnique` (`self.ItemPool`) _output_get)))
  (`/Game/BluePrints/Objects/Item/BP_Item.Item_GetUp` _local_accessible_item Item_RowName)
  (`self.K2_TeleportTo` :`self` _local_accessible_item :`DestLocation` DestLocation))

(fn `Awake_A_Monster`
  (params (Monster_RowName :type Name) (Location :type "Vector Structure"))
  (locals (Local_Accessible_Monster :type "/Game/BluePrints/Entities/Monsters/BP_Monster Object Reference"))
  (bind _local_accessible_monster (`local.Local_Accessible_Monster`))
  (for _array_element (`self.MonsterPool`)
    (if (`|EnumEquality` (`/Game/BluePrints/Entities/Monsters/BP_Monster.Monster_State` _array_element) "NewEnumerator1")
      (set `local.Local_Accessible_Monster` _array_element)
      (break)))
  (`local.Local_Accessible_Monster`
    (:`then`
      _)
    (:`else`
      (bind _returnvalue (`|SpawnActorFromClass` "/Game/BluePrints/Entities/Monsters/BP_Monster.BP_Monster_C" (`KismetMathLibrary.MakeTransform` (0.0 0.0 50000.0)) "Undefined" "MultiplyWithRoot" null Monster_RowName null))
      (bind _output_get (set `local.Local_Accessible_Monster` _returnvalue))
      (`KismetArrayLibrary.Array_AddUnique` (`self.MonsterPool`) _output_get)))
  (`/Game/BluePrints/Entities/Monsters/BP_Monster.Monster_GetUp` _local_accessible_monster Monster_RowName)
  (`self.K2_TeleportTo` :`self` _local_accessible_monster :`DestLocation` Location)
  (`KismetArrayLibrary.Array_Add` (`self.MonsterPool_Awake`) _local_accessible_monster))

(fn `Awake_A_Object`
  (params (Object_Type :type "/Game/BluePrints/Objects/E_ObjectType Enum" :default "NewEnumerator6") (Object_RowName :type Name) (DestLocation :type "Vector Structure"))
  (locals (Local_Accessible_Object :type "/Game/BluePrints/Objects/BP_Object Object Reference"))
  (bind _local_accessible_object (`local.Local_Accessible_Object`))
  (for _array_element (`self.ObjectPool`)
    (if (`|EnumEquality` (`/Game/BluePrints/Objects/BP_Object.Object_State` _array_element) "NewEnumerator1")
      (set `local.Local_Accessible_Object` _array_element)
      (break)))
  (`local.Local_Accessible_Object`
    (:`then`
      _)
    (:`else`
      (bind _returnvalue (`|SpawnActorFromClass` "/Game/BluePrints/Objects/BP_Object.BP_Object_C" (`KismetMathLibrary.MakeTransform` (0.0 0.0 50000.0)) "Undefined" "MultiplyWithRoot" null Object_Type Object_RowName null)) ; 没有可用对象则生成对象
      (bind _output_get (set `local.Local_Accessible_Object` _returnvalue))
      (`KismetArrayLibrary.Array_AddUnique` (`self.ObjectPool`) _output_get)))
  (`/Game/BluePrints/Objects/BP_Object.Object_GetUp` _local_accessible_object Object_Type Object_RowName)
  (bind _returnvalue_2 (`self.K2_TeleportTo` :`self` _local_accessible_object :`DestLocation` DestLocation))
  (if _returnvalue_2
    (`/Game/BluePrints/Objects/BP_Object.ObjectJump` _local_accessible_object)))

(fn `Awake_A_Summon`
  (params (Summon_RowName :type Name) (Called_Position :type "Vector Structure") (Launch_Direction :type "Vector Structure") (Caller_Tag :type Name) (Caller_MagicPower :type Integer))
  (returns (Sussess :type Boolean))
  (locals (Local_Accessible_Summon :type "/Game/BluePrints/Objects/Summon/BP_Summon Object Reference"))
  (bind _local_accessible_summon (`local.Local_Accessible_Summon`))
  (if (< (`KismetArrayLibrary.Array_Length` (`self.Summon_Pool_Awake`)) (`self.Max_Summon_Num`))
    (for _array_element (`self.Summon_Pool`)
      (if (`|EnumEquality` (`/Game/BluePrints/Objects/Summon/BP_Summon.Summon_State` _array_element) "NewEnumerator1")
        (set `local.Local_Accessible_Summon` _array_element)
        (break)))
    (`local.Local_Accessible_Summon`
      (:`then`
        _)
      (:`else`
        (bind _returnvalue (`|SpawnActorFromClass` "/Game/BluePrints/Objects/Summon/BP_Summon.BP_Summon_C" (`KismetMathLibrary.MakeTransform` (0.0 0.0 50000.0)) "Undefined" "MultiplyWithRoot" null "None" "(INVALID)" "None" 0 null)) ; 没有可用对象则生成对象
        (bind _output_get (set `local.Local_Accessible_Summon` _returnvalue))
        (`KismetArrayLibrary.Array_AddUnique` (`self.Summon_Pool`) _output_get)))
    (`/Game/BluePrints/Objects/Summon/BP_Summon.Summon_GetUp` _local_accessible_summon Summon_RowName Launch_Direction Caller_Tag Caller_MagicPower)
    (`self.K2_TeleportTo` :`self` _local_accessible_summon :`DestLocation` Called_Position)
    (`KismetArrayLibrary.Array_Add` (`self.Summon_Pool_Awake`) _local_accessible_summon)
    (return true)
    (else
      (return false))))

(fn `Awake_Num_Item`
  (params (Item_RowName :type Name) (Num :type Integer) (Location :type "Vector Structure (by ref)") (Radius :type "Float (double-precision)"))
  (bind (_world_x _world_y) (`/Game/Instance/Public/FL_Public.Get_RandomLocation_AroundPoint` (`KismetMathLibrary.MakeVector2D` (.x Location) (.y Location)) Radius))
  (for _ (range 1 (+ Num 1))
    (`self.Awake_A_Item` Item_RowName (`KismetMathLibrary.MakeVector_NetQuantize` _world_x _world_y 10.0)))
  (return))

(fn `Awake_Num_Object`
  (params (Object_Type :type "/Game/BluePrints/Objects/E_ObjectType Enum" :default "NewEnumerator6") (Object_RowName :type Name) (Num :type Integer) (Location :type "Vector Structure (by ref)") (Radius :type "Float (single-precision)"))
  (bind (_world_x _world_y) (`/Game/Instance/Public/FL_Public.Get_RandomLocation_AroundPoint` (`KismetMathLibrary.MakeVector2D` (.x Location) (.y Location)) Radius))
  (for _ (range 1 (+ Num 1))
    (`self.Awake_A_Object` Object_Type Object_RowName (`KismetMathLibrary.MakeVector_NetQuantize` _world_x _world_y 10.0)))
  (return))

(fn `Character_Awake_A_Projectile`
  (params (Projectile_RowName :type Name) (Launch_Position :type "Vector Structure") (Launch_Direction :type "Vector Structure") (Shooter_Tag :type Name) (Shooter_Power :type Integer) (BP_EffectsAreas :type "/Game/BluePrints/Sences/BP_EffectsArea Object Reference"))
  (returns (Sussess :type Boolean))
  (locals (Local_Accessible_Projectile :type "/Game/BluePrints/Objects/Projectile/BP_Projectile Object Reference"))
  (bind _local_accessible_projectile (`local.Local_Accessible_Projectile`))
  (if (< (`KismetArrayLibrary.Array_Length` (`self.Character_ProjectilePool_Awake`)) (`self.Character_Max_Projectile_Num`))
    (for _array_element (`self.Character_ProjectilePool`)
      (if (`|EnumEquality` (`/Game/BluePrints/Objects/Projectile/BP_Projectile.Projectile_State` _array_element) "NewEnumerator1")
        (set `local.Local_Accessible_Projectile` _array_element)
        (break)))
    (`local.Local_Accessible_Projectile`
      (:`then`
        _)
      (:`else`
        (bind _returnvalue (`|SpawnActorFromClass` "/Game/BluePrints/Objects/Projectile/BP_Projectile.BP_Projectile_C" (`KismetMathLibrary.MakeTransform` (0.0 0.0 50000.0)) "Undefined" "MultiplyWithRoot" null "None" null)) ; 没有可用对象则生成对象
        (bind _output_get (set `local.Local_Accessible_Projectile` _returnvalue))
        (`KismetArrayLibrary.Array_AddUnique` (`self.Character_ProjectilePool`) _output_get)))
    (`/Game/BluePrints/Objects/Projectile/BP_Projectile.Projectile_GetUp` _local_accessible_projectile Projectile_RowName Launch_Direction Shooter_Tag Shooter_Power BP_EffectsAreas)
    (`self.K2_TeleportTo` :`self` _local_accessible_projectile :`DestLocation` Launch_Position)
    (`KismetArrayLibrary.Array_Add` (`self.Character_ProjectilePool_Awake`) _local_accessible_projectile)
    (return true)
    (else
      (return false))))

(fn `DEBUG_Print_PoolNum`
  (`KismetSystemLibrary.PrintText` (`|FormatText` "MonsterPool:{A}/{B}" (`KismetArrayLibrary.Array_Length` (`self.MonsterPool_Awake`)) (`KismetArrayLibrary.Array_Length` (`self.MonsterPool`))) true true (struct :`G` 0.66 :`B` 1.0 :`A` 1.0) 0.0)
  (`KismetSystemLibrary.PrintText` (`|FormatText` "ProjectilePool:{A}/{B} \nMonster_ProjectilePool:{C}" (`KismetArrayLibrary.Array_Length` (`self.Character_ProjectilePool_Awake`)) (`KismetArrayLibrary.Array_Length` (`self.Character_ProjectilePool`)) (`KismetArrayLibrary.Array_Length` (`self.Monster_ProjectilePool`))) true true (struct :`G` 0.66 :`B` 1.0 :`A` 1.0) 0.0)
  (`KismetSystemLibrary.PrintText` (`|FormatText` "SummonPool:{A}/{B}" (`KismetArrayLibrary.Array_Length` (`self.Summon_Pool_Awake`)) (`KismetArrayLibrary.Array_Length` (`self.Summon_Pool`))) true true (struct :`G` 0.66 :`B` 1.0 :`A` 1.0) 0.0)
  (`KismetSystemLibrary.PrintText` (`|FormatText` "ItemPool:{A}" (`KismetArrayLibrary.Array_Length` (`self.ItemPool`))) true true (struct :`G` 0.66 :`B` 1.0 :`A` 1.0) 0.0)
  (`KismetSystemLibrary.PrintText` (`|FormatText` "ObjectPool:{A}" (`KismetArrayLibrary.Array_Length` (`self.ObjectPool`))) true true (struct :`G` 0.66 :`B` 1.0 :`A` 1.0) 0.0)
  (if (`self.Character_Is_Update_ProjectileNum`)
    (`/Game/UI/InGameHUD/WB_UI_HUD_InGame.Update_Projectile_Num` (`/Game/BluePrints/Entities/Characters/BP_Character.WB_UI_HUD_InGame` (`/Game/Instance/Public/FL_Public.Get_Character`)) (`KismetArrayLibrary.Array_Length` (`self.Character_ProjectilePool_Awake`)) (`self.Character_Max_Projectile_Num`))
    (if (`self.Is_Update_SummonNum`)
      (`/Game/UI/InGameHUD/WB_UI_HUD_InGame.Update_Summon_Num` (`/Game/BluePrints/Entities/Characters/BP_Character.WB_UI_HUD_InGame` (`/Game/Instance/Public/FL_Public.Get_Character`)) (`KismetArrayLibrary.Array_Length` (`self.Summon_Pool_Awake`)) (`self.Max_Summon_Num`)))))

(fn `Get Random Out Viewport Spawn Location`
  (returns (Random_OutViewport_SpawnLocation :type "Vector Structure"))
  (locals (RandomLocation :type "Vector Structure" :default (0.0 0.0 0.0)))
  (bind (_randomlocation _returnvalue) (`NavigationSystemV1.K2_GetRandomLocationInNavigableRadius` (`self.K2_GetActorLocation` (`GameplayStatics.GetPlayerPawn` 0)) 10000.0 null null :!label _label))
  (if _returnvalue
    (bind _output_get (set `local.RandomLocation` (`KismetMathLibrary.MakeVector` (.x _randomlocation) (.y _randomlocation) 10.0)))
    (if (`/Game/Instance/Public/FL_Public.Check_Is_In_Viewport` _output_get)
      (goto _label)
      (else
        (return (`local.RandomLocation`))))
    (else
      (`/Game/Instance/Public/FL_Public.DEBUG_MYLOG` "NewEnumerator2" "Get RandomLocation Failed" "BP_ActorPool" "Get Random Out Viewport Spawn Location"))))

(fn `Get_Random_AroundActor_SpawnLocation`
  (params (ActorLocation :type "Vector Structure (by ref)") (Radius :type "Float (single-precision)"))
  (returns (Random_AroundLocation_SpawnLocation :type "Vector Structure"))
  (bind _randomlocation (`NavigationSystemV1.K2_GetRandomLocationInNavigableRadius` ActorLocation Radius null null))
  (return _randomlocation))

(fn `Init_DataAssets`
  (`self.Init_Projectile_DataAsset_All` true)
  (`self.Init_Summon_DataAsset_All` true)
  (`self.Init_Surround_DataAsset_All` true)
  (`self.Init_Monster_DataAsset_All` true))

(fn `Init_Monster_DataAsset_All`
  (params (Is_From_DT_DA_Init :type Boolean) (Is_From_Profile :type Boolean))
  (if Is_From_DT_DA_Init
    (bind _outrownames (`DataTableFunctionLibrary.GetDataTableRowNames` "/Game/BluePrints/Entities/Monsters/DT_Monster.DT_Monster")) ; 因为Monster在游戏开始时并未设置具体RowName,\n所以初始化DA时需要将所有Monster的DA都初始化，\n或许有更好的解决方案，但暂时先这样处理
    (for _array_element _outrownames
      (bind _returnvalue (`|GetDataTableRow` "/Game/BluePrints/Entities/Monsters/DT_Monster.DT_Monster" _array_element)
        (:`then`
          (`/Game/BluePrints/Entities/Monsters/DataAssets/BP_DA_Monster.Init_DataAsset` (`.DataAsset_11_3A16B7204895299A20C03C8B231E2B82` (break `/Game/BluePrints/Entities/Monsters/S_Monster` _returnvalue)) _array_element))))
    (return)
    (else
      ;[1 1 1] TODO
      (if Is_From_Profile
        _))))

(fn `Init_Projectile_DataAsset_All`
  (params (Is_From_DT_DA_Init :type Boolean) (Is_From_Profile :type Boolean))
  (if Is_From_DT_DA_Init
    (bind _outrownames (`DataTableFunctionLibrary.GetDataTableRowNames` "/Game/BluePrints/Objects/Projectile/DT_Projectile.DT_Projectile")) ; 因为Projectile在游戏开始时并未设置具体RowName,\n只有在发射的时候才拥有RowName，\n所以初始化DA时需要将所有Projectile的DA都初始化，\n或许有更好的解决方案，但暂时先这样处理
    (for _array_element _outrownames
      (bind _returnvalue (`|GetDataTableRow` "/Game/BluePrints/Objects/Projectile/DT_Projectile.DT_Projectile" _array_element)
        (:`then`
          (`/Game/BluePrints/Objects/Projectile/DataAssets/BP_DA_Projectile.Init_DataAsset` (`.DataAsset_6_7622AA0049E3DCE69AE0F98C630F881B` (break `/Game/BluePrints/Objects/Projectile/S_Projectile` _returnvalue)) _array_element))))
    (return)
    (else
      ;[1 1 1] TODO
      (if Is_From_Profile
        _))))

(fn `Init_Summon_DataAsset_All`
  (params (Is_From_DT_DA_Init :type Boolean) (Is_From_Profile :type Boolean))
  (if Is_From_DT_DA_Init
    (bind _outrownames (`DataTableFunctionLibrary.GetDataTableRowNames` "/Game/BluePrints/Objects/Summon/DT_Summon.DT_Summon")) ; 因为Summon在游戏开始时并未设置具体RowName,\n只有在发射的时候才拥有RowName，\n所以初始化DA时需要将所有Summon的DA都初始化，\n或许有更好的解决方案，但暂时先这样处理
    (for _array_element _outrownames
      (bind _returnvalue (`|GetDataTableRow` "/Game/BluePrints/Objects/Summon/DT_Summon.DT_Summon" _array_element)
        (:`then`
          (`/Game/BluePrints/Objects/Summon/DataAsset/BP_DA_Summon.Init_DataAsset` (`.DataAsset_8_0B3C256242BA53DD7C2BF794213BD4D3` (break `/Game/BluePrints/Objects/Summon/S_Summon` _returnvalue)) _array_element))))
    (return)
    (else
      ;[1 1 1] TODO
      (if Is_From_Profile
        _))))

(fn `Init_Surround_DataAsset_All`
  (params (Is_From_DT_DA_Init :type Boolean) (Is_From_Profile :type Boolean))
  (if Is_From_DT_DA_Init
    (bind _outrownames (`DataTableFunctionLibrary.GetDataTableRowNames` "/Game/BluePrints/Objects/Surround/DT_Surround.DT_Surround")) ; 因为Surround在游戏开始时并未设置具体RowName,\n只有在发射的时候才拥有RowName，\n所以初始化DA时需要将所有Surround的DA都初始化，\n或许有更好的解决方案，但暂时先这样处理
    (for _array_element _outrownames
      (bind _returnvalue (`|GetDataTableRow` "/Game/BluePrints/Objects/Surround/DT_Surround.DT_Surround" _array_element)
        (:`then`
          (`/Game/BluePrints/Objects/Surround/DataAssets/BP_DA_Surround.Surround_init_DataAsset` (`.DataAsset_5_F98685DA400D10DA89818991F0241283` (break `/Game/BluePrints/Objects/Surround/S_Surround` _returnvalue)) _array_element))))
    (return)
    (else
      ;[1 1 1] TODO
      (if Is_From_Profile
        _))))

(fn `Monster_Awake_A_Projectile`
  (params (Projectile_RowName :type Name) (Launch_Position :type "Vector Structure") (Launch_Direction :type "Vector Structure") (Shooter_Tag :type Name) (Shooter_Power :type Integer))
  (returns (Sussess :type Boolean))
  (locals (Local_Accessible_Projectile :type "/Game/BluePrints/Objects/Projectile/BP_Projectile Object Reference"))
  (bind _local_accessible_projectile (`local.Local_Accessible_Projectile`))
  (for _array_element (`self.Monster_ProjectilePool`)
    (if (`|EnumEquality` (`/Game/BluePrints/Objects/Projectile/BP_Projectile.Projectile_State` _array_element) "NewEnumerator1")
      (set `local.Local_Accessible_Projectile` _array_element)
      (break)))
  (`local.Local_Accessible_Projectile`
    (:`then`
      _)
    (:`else`
      (bind _returnvalue (`|SpawnActorFromClass` "/Game/BluePrints/Objects/Projectile/BP_Projectile.BP_Projectile_C" (`KismetMathLibrary.MakeTransform` (0.0 0.0 50000.0)) "Undefined" "MultiplyWithRoot" null "None" null)) ; 没有可用对象则生成对象
      (bind _output_get (set `local.Local_Accessible_Projectile` _returnvalue))
      (`KismetArrayLibrary.Array_AddUnique` (`self.Monster_ProjectilePool`) _output_get)))
  (`/Game/BluePrints/Objects/Projectile/BP_Projectile.Projectile_GetUp` _local_accessible_projectile Projectile_RowName Launch_Direction Shooter_Tag Shooter_Power null)
  (bind _returnvalue_2 (`self.K2_TeleportTo` :`self` _local_accessible_projectile :`DestLocation` Launch_Position))
  (return _returnvalue_2))

(fn `Spawn Character`
  (bind _returnvalue (`|SpawnActorFromClass` "/Game/BluePrints/Entities/Characters/BP_Character.BP_Character_C" (`KismetMathLibrary.MakeTransform` (`self.Character_Location`)) "Undefined" "MultiplyWithRoot" self "Boy" null))
  (bind _output_get (set `self.BP_Character` _returnvalue))
  (`Controller.Possess` (`GameplayStatics.GetPlayerController` 0) _output_get)
  (`KismetSystemLibrary.PrintString` "Create Character" true true (struct :`R` 1.0 :`B` 0.602382 :`A` 1.0)))

(fn `TryTo_Fillup_MonsterPool`
  (if (< (`KismetArrayLibrary.Array_Length` (`self.MonsterPool_Awake`)) (`KismetArrayLibrary.Array_Length` (`self.MonsterPool`)))
    (bind _random_outviewport_spawnlocation (`self.Get Random Out Viewport Spawn Location`))
    (bind _outrownames (`DataTableFunctionLibrary.GetDataTableRowNames` "/Game/BluePrints/Entities/Monsters/DT_Monster.DT_Monster"))
    (`self.Awake_A_Monster` (`KismetArrayLibrary.Array_Random` _outrownames) _random_outviewport_spawnlocation)))

(fn `UserConstructionScript`)