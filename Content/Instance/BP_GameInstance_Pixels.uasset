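; BP_GameInstance_Pixels is the game instance, handling restarts and an elapsed-time counter for the in-game HUD.
; Restart sets a restart flag and forwards the call to the character.
; Timer_Start creates a looping one-second timer, first clearing the old one and zeroing the count if that flag is set.
; Timer_Count increments the counter and sends minutes and seconds to the character's HUD widget.
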(event `self.ReceiveInit`)

(event `Restart`
  (set `self.Is_Restart` true)
  (`/Game/BluePrints/Entities/Characters/BP_Character.Restart` (`/Game/Instance/Public/FL_Public.Get_Character`)))

(event `Timer_Start`
  (if (`self.Is_Restart`)
    (`KismetSystemLibrary.K2_ClearAndInvalidateTimerHandle` (`self.Game_Timer`))
    (set `self.Time_Counter` 0))
  (bind _returnvalue (`KismetSystemLibrary.K2_SetTimerDelegate` (`|CreateDelegate` :!event `Timer_Count`) 1.0 true))
  (set `self.Game_Timer` _returnvalue))

(event `Timer_Count`
  (bind _result (`/Engine/EditorBlueprintResources/StandardMacros.IncrementInt` (`self.Time_Counter`))
    (:`  `
      (`/Game/UI/InGameHUD/WB_UI_HUD_InGame.Update_Timer` (`/Game/BluePrints/Entities/Characters/BP_Character.WB_UI_HUD_InGame` (`/Game/Instance/Public/FL_Public.Get_Character`)) true (/ _result 60) (mod _result 60)))))