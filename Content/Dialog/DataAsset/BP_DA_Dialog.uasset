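; Dialog data asset holding branching Talks and Replys, with a cursor that tracks the current position in the conversation.
; DialogLocation is an IntVector indexing the nested arrays, and IsReply marks whether a reply choice is active.
; Continue reads the event from the current line or chosen reply, then advances, jumps to another talk or switches to replies.
; It returns whether to hide the dialog; fight, store and item events only end it here.
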(fn `Continue`
  (params (S_ReplyContent :type "/Game/Dialog/S_ReplyContent Structure"))
  (returns (Is_HideDialog :type Boolean))
  (locals (Local_Event :type "/Game/Dialog/E_Event Enum") (Local_Index :type Integer) (Local_IS_HideDialog :type Boolean :default true))
  (bind ((`E_Event_5_464873A3431A2454E9942D9C7E24F657` _e_event) (`Next_Talk_OR_Reply_Index_10_BFBD151546E688BC71C7089550326620` _next_talk_or_reply_index)) (break `/Game/Dialog/S_ReplyContent` S_ReplyContent))
  (bind _dialog_location_x (break `IntVector` (`self.Dialog_Location`)))
  (bind (_dialog_location_x_2 _dialog_location_y _dialog_location_z) (break `IntVector` (`self.Dialog_Location`)))
  (bind ((`E_Event_12_61ABFBBC411E730D1D40549D87079186` _e_event_2) (`Next_Talk_OR_Reply_Index_30_C49CAAFA46B3BD6563F87EA8A0CB62C9` _next_talk_or_reply_index_2)) (break `/Game/Dialog/S_TalkContent` (`self.Get_Current_Talk_Content`)))
  (if (`self.Is_Reply`)
    (set `local.Local_Event` _e_event)
    (set `local.Local_Index` _next_talk_or_reply_index)
    (else
      (set `local.Local_Event` _e_event_2)
      (set `local.Local_Index` _next_talk_or_reply_index_2)))
  (switch `/Game/Dialog/E_Event` (`local.Local_Event`)
    (:`NewEnumerator5`
      (set `self.Dialog_Location` (make `IntVector` _dialog_location_x_2 _dialog_location_y (+ _dialog_location_z 1)))
      (set `self.Is_Reply` false :!label _label)
      (set `local.Local_IS_HideDialog` false))
    (:`NewEnumerator8`
      (set `self.Dialog_Location` (make `IntVector` (`local.Local_Index`)))
      (goto _label))
    (:`NewEnumerator7`
      (set `self.Is_Reply` true)
      (set `local.Local_IS_HideDialog` false)
      (set `self.Dialog_Location` (make `IntVector` _dialog_location_x) :!label _label_2))
    (:`NewEnumerator6`
      (set `local.Local_IS_HideDialog` true :!label _label_3)
      (goto _label_2))
    (:`NewEnumerator2`
      (goto _label_3))
    (:`NewEnumerator1`
      (goto _label_3))
    (:`NewEnumerator4`
      (goto _label_3)))
  (return (`local.Local_IS_HideDialog`)))

(fn `Get_Current_Reply_Content`
  (returns (Question :type Text) (ReplyContents :type "Array of /Game/Dialog/S_ReplyContent Structure"))
  (bind (_x _y) (break `IntVector` (`self.Dialog_Location`)))
  (bind (_question _replycontent) (break `/Game/Dialog/S_ReplyGroup` (`|GetArrayItem` (`.ReplyGroup_4_998097CD48EF55407E9721B0C0EEEE70` (break `/Game/Dialog/S_Reply` (`|GetArrayItem` (`self.Replys`) _x))) _y)))
  (return _question _replycontent))

(fn `Get_Current_Talk_Content`
  (returns (TalkContent :type "/Game/Dialog/S_TalkContent Structure"))
  (bind (_x _y _z) (break `IntVector` (`self.Dialog_Location`)))
  (return (`|GetArrayItem` (`.TalkContent_6_20A60DB947B1267AD5C61FB95451D9A8` (break `/Game/Dialog/S_TalkGroup` (`|GetArrayItem` (`.TalkGroup_4_1D6FE27D4631CDAECA660D8B4C96D7CC` (break `/Game/Dialog/S_Talk` (`|GetArrayItem` (`self.Talks`) _x))) _y))) _z)))

(fn `Init_DataAsset`
  (set `self.Is_Reply` false)
  (set `self.Dialog_Location` (make `IntVector` 0))
  (return))