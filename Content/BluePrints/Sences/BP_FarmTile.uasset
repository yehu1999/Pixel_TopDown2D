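; Farm tile actor that handles planting, watering, crop growth and harvesting with Paper2D sprites.
; Plant resolves a seed to its crop via data tables; while planted and watered, Tick runs a looping countdown timer that advances staged sprites and yields until ripe.
; Water wears off after a retriggerable delay, and Feed's delay also clears the watered flag.
; Harvest clears the crop, waking pooled drops if ripe.
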(event `self.ReceiveTick`
  (params (DeltaSeconds :type "Float (single-precision)"))
  (if (and (not (`self.Is_Crop_Ripe`)) (not (`self.Is_Crop_Growing`)) (`self.Is_Tile_Planted`) (`self.Is_Tile_Watered`))
    (set `self.Is_Crop_Growing` true)
    (bind _returnvalue (`KismetSystemLibrary.K2_SetTimerDelegate` (delegate `Crop_Growing`) 1.0 true))
    (set `self.Timer_Growing` _returnvalue)
    (elif (or (not (`self.Is_Tile_Planted`)) (not (`self.Is_Tile_Watered`)))
      (`KismetSystemLibrary.K2_ClearAndInvalidateTimerHandle` (`self.Timer_Growing`))
      (set `self.Is_Crop_Growing` false))))

(event `Crop_Growing`
  (bind _result (`/Engine/EditorBlueprintResources/StandardMacros.DecrementInt` (`self.Crop_GrowingTime`))
    (:`  `
      (if (<= _result 0)
        (`self.Crop_GrowUp`)))))

(event `Plant`
  (params (Crop_RowName :type Name))
  (if (not (`self.Is_Tile_Planted`))
    (bind _returnvalue (`|GetDataTableRow` "/Game/BluePrints/Objects/Seed/DT_Seed.DT_Seed" Crop_RowName)
      (:`then`
        (bind ((`Crop_RowName_11_09CD17AA4883A85EC80C3DB01B5F414E` _crop_rowname)) (break `/Game/BluePrints/Objects/Seed/S_Seed` _returnvalue))
        (bind _returnvalue_2 (`|GetDataTableRow` "/Game/BluePrints/Objects/Crop/DT_Crop.DT_Crop" _crop_rowname)
          (:`then`
            (set `self.Crop_RowName` _crop_rowname)
            (set `self.Is_Tile_Planted` true)
            (bind ((`Crop_Sprite_0_15_0DAB28F047A37A1887C5E78130161772` _crop_sprite_0) (`GrowingTime_01_21_792B9CDB409459080624D6843D7B5F43` _growingtime_01)) (break `/Game/BluePrints/Objects/Crop/S_Crop` _returnvalue_2))
            (`PaperSpriteComponent.SetSprite` (`self.PaperSprite_Crop`) _crop_sprite_0)
            (`SceneComponent.SetVisibility` (`self.PaperSprite_Crop`) true false)
            (set `self.Crop_GrowingTime` _growingtime_01)
            (set `self.Crop_GrowingLevel` 0)
            (set `self.Crop_Amount` 0)
            (set `self.Is_Crop_Growing` false)
            (set `self.Is_Crop_Ripe` false)))))))

(event `Harvest`
  (if (`self.Is_Crop_Ripe`)
    (`/Game/Instance/BP_ActorPool.Awake_Num_Object` (`/Game/Instance/Public/FL_Public.Get_ActorPool`) "NewEnumerator1" (`self.Crop_RowName`) (`self.Crop_Amount`) (`self.K2_GetActorLocation`) 16.0))
  (`SceneComponent.SetVisibility` (`self.PaperSprite_Crop`) false false)
  (set `self.Is_Tile_Planted` false)
  (set `self.Is_Crop_Ripe` false)
  (set `self.Crop_RowName` "None"))

(event `Water`
  (set `self.Is_Tile_Watered` true)
  (`PaperSpriteComponent.SetSprite` (`self.PaperSprite_FarmTile`) "/Game/Sprites_Anims/Sence/FarmTile/Sprite_FarmTile_Wet.Sprite_FarmTile_Wet")
  (`KismetSystemLibrary.RetriggerableDelay` 25.0) ; 浇水有效时间
  (`PaperSpriteComponent.SetSprite` (`self.PaperSprite_FarmTile`) "/Game/Sprites_Anims/Sence/FarmTile/Sprite_FarmTile_Dry.Sprite_FarmTile_Dry")
  (set `self.Is_Tile_Watered` false))

(event `Feed`
  (set `self.Is_Tile_Fed` true)
  (`KismetSystemLibrary.RetriggerableDelay` 3.0)
  (set `self.Is_Tile_Watered` false))

(fn `Crop_GrowUp`
  (locals (Local_CropSprite :type "PaperSprite Object Reference"))
  (bind _crop_rowname (`self.Crop_RowName`))
  (bind _result (`/Engine/EditorBlueprintResources/StandardMacros.IncrementInt` (`self.Crop_GrowingLevel`))
    (:`  `
      (switch `int` _result
        (:`0`
          (bind _returnvalue (`|GetDataTableRow` "/Game/BluePrints/Objects/Crop/DT_Crop.DT_Crop" _crop_rowname)
            (:`then`
              (bind ((`Crop_Sprite_0_15_0DAB28F047A37A1887C5E78130161772` _crop_sprite_0) (`Crop_Sprite_Harvested_41_1B3206D64117402A466495B20EC9F4CC` _crop_sprite_harvested) (`GrowingTime_01_21_792B9CDB409459080624D6843D7B5F43` _growingtime_01) (`CropAmount_0_32_E5EBC6DD41B7C6DAFF3F5E930DB0A73F` _cropamount_0)) (break `/Game/BluePrints/Objects/Crop/S_Crop` _returnvalue))
              (set `local.Local_CropSprite` _crop_sprite_0)
              (set `self.Crop_GrowingTime` _growingtime_01)
              (set `self.Crop_Amount` _cropamount_0))))
        (:`1`
          (bind _returnvalue_2 (`|GetDataTableRow` "/Game/BluePrints/Objects/Crop/DT_Crop.DT_Crop" _crop_rowname)
            (:`then`
              (bind ((`Crop_Sprite_1_16_479DB3E6487E4FA63D581D96CC3B1681` _crop_sprite_1) (`Crop_Sprite_Harvested_41_1B3206D64117402A466495B20EC9F4CC` _crop_sprite_harvested_2) (`GrowingTime_12_23_FDED4B894F2A398C9088878316C03957` _growingtime_12) (`CropAmount_1_34_1F0E23B145E6791DFBF5109AA2B1F8A3` _cropamount_1)) (break `/Game/BluePrints/Objects/Crop/S_Crop` _returnvalue_2))
              (set `local.Local_CropSprite` _crop_sprite_1)
              (set `self.Crop_GrowingTime` _growingtime_12)
              (set `self.Crop_Amount` _cropamount_1))))
        (:`2`
          (bind _returnvalue_3 (`|GetDataTableRow` "/Game/BluePrints/Objects/Crop/DT_Crop.DT_Crop" _crop_rowname)
            (:`then`
              (bind ((`Crop_Sprite_2_17_7F9A73B344D455F96DC8DD966970FA08` _crop_sprite_2) (`Crop_Sprite_Harvested_41_1B3206D64117402A466495B20EC9F4CC` _crop_sprite_harvested_3) (`GrowingTime_23_25_2177C4104F4762F7CC9A6B9C1C81B60B` _growingtime_23) (`CropAmount_2_36_BF65B9A04081831EA37100A79CFEA923` _cropamount_2)) (break `/Game/BluePrints/Objects/Crop/S_Crop` _returnvalue_3))
              (set `local.Local_CropSprite` _crop_sprite_2)
              (set `self.Crop_GrowingTime` _growingtime_23)
              (set `self.Crop_Amount` _cropamount_2))))
        (:`3`
          (bind _returnvalue_4 (`|GetDataTableRow` "/Game/BluePrints/Objects/Crop/DT_Crop.DT_Crop" _crop_rowname)
            (:`then`
              (bind ((`Crop_Sprite_3_18_0CA7E0BC4F819D9C6B949F8306B93C71` _crop_sprite_3) (`Crop_Sprite_Harvested_41_1B3206D64117402A466495B20EC9F4CC` _crop_sprite_harvested_4) (`CropAmount_3_38_7F98BCC74ABD3104A4D1C2BFD73916AB` _cropamount_3)) (break `/Game/BluePrints/Objects/Crop/S_Crop` _returnvalue_4))
              (set `local.Local_CropSprite` _crop_sprite_3)
              (set `self.Crop_Amount` _cropamount_3)))))
      (`PaperSpriteComponent.SetSprite` (`self.PaperSprite_Crop`) (`local.Local_CropSprite`))
      (if (== (`self.Crop_GrowingLevel`) 3)
        (set `self.Is_Crop_Growing` false)
        (set `self.Is_Crop_Ripe` true)
        (`KismetSystemLibrary.K2_ClearAndInvalidateTimerHandle` (`self.Timer_Growing`))))))

(fn `Get_Object_Info`
  (returns (Object_Type :type "/Game/BluePrints/Objects/E_ObjectType Enum") (Object_RowName :type Name))
  (return "NewEnumerator6" "None"))

(fn `UserConstructionScript`)