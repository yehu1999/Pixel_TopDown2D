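; BP_Home is a destructible home base that lures AI by reporting a "Home"-tagged noise every tick while its HP remains.
; Box overlaps with living monsters or any projectile cost one HP and refresh the widget life bar.
; Each hit briefly disables box collision as a damage cooldown; at zero HP collision stays off and the Paper2D sprite is swapped.
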(event `self.ReceiveTick`
  (params (DeltaSeconds :type "Float (single-precision)"))
  (if (> (`self.HP`) 0)
    (`AISense_Hearing.ReportNoiseEvent` (`self.K2_GetActorLocation`) 1.0 self 0.0 "Home") ; 产生噪音（刺激AI听觉）
  ))

(event `self.Box.OnComponentBeginOverlap`
  (params (OverlappedComponent :type "PrimitiveComponent Object Reference") (OtherActor :type "Actor Object Reference") (OtherComp :type "PrimitiveComponent Object Reference") (OtherBodyIndex :type Integer) (bFromSweep :type Boolean) (SweepResult :type "HitResult Structure (by ref)"))
  (bind _asbp_monster (cast `/Game/BluePrints/Entities/Monsters/BP_Monster` OtherActor)
    (:`then`
      (if (`/Game/BluePrints/Entities/Monsters/BP_Monster.Get_Is_Alive` _asbp_monster)
        (`/Engine/EditorBlueprintResources/StandardMacros.DecrementInt` (`self.HP`)
          (:`  `
            (`self.Update_LifeBar` :!label _label)
            (`PrimitiveComponent.SetCollisionEnabled` (`self.Box`) "NoCollision")
            (if (> (`self.HP`) 0)
              (`KismetSystemLibrary.Delay` 0.5)
              (`PrimitiveComponent.SetCollisionEnabled` (`self.Box`) "QueryOnly")
              (else
                (`PaperSpriteComponent.SetSprite` (`self.PaperSprite_Home`) "/Game/Sprites_Anims/Object/Crops/Crop_Spritesheet_Sprite_74.Crop_Spritesheet_Sprite_74")))))))
    (:`CastFailed`
      (bind _asbp_projectile (cast `/Game/BluePrints/Objects/Projectile/BP_Projectile` OtherActor))
      (if true
        (`/Engine/EditorBlueprintResources/StandardMacros.DecrementInt` (`self.HP`)
          (:`  `
            (goto _label)))))))

(event `Update_LifeBar`
  (bind _aswb_life_bar (cast `/Game/UI/WB_LifeBar` (`WidgetComponent.GetWidget` (`self.Widget_LifeBar`))))
  (`/Game/UI/WB_LifeBar.Update` _aswb_life_bar (`self.HP`) 10))

(fn `UserConstructionScript`)