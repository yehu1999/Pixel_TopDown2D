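; BP_Store is a store actor that hosts a merchant NPC through the ChildActorMerchant child actor component.
; It casts the child actor to BP_NPC and passes NPCRowName to NPCSetupBaseData to set up the merchant's base data.
; This setup runs in the construction script and again on BeginPlay, while the overlap and tick events are empty.
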(event `self.ReceiveBeginPlay`
  (bind _asbp_npc (cast `/Game/BluePrints/Entities/NPC/BP_NPC` (`ChildActorComponent.ChildActor` (`self.ChildActor_Merchant`))))
  (`/Game/BluePrints/Entities/NPC/BP_NPC.NPC_Setup_BaseData` _asbp_npc (`self.NPC_RowName`)))

(fn `UserConstructionScript`
  (bind _asbp_npc (cast `/Game/BluePrints/Entities/NPC/BP_NPC` (`ChildActorComponent.ChildActor` (`self.ChildActor_Merchant`))))
  (`/Game/BluePrints/Entities/NPC/BP_NPC.NPC_Setup_BaseData` _asbp_npc (`self.NPC_RowName`)))