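; BP_Rotater spins a ring of BP_Surround actors, centred on its parent actor's location when built.
; CreateSurrounds reads radius and yaw rate from a DT_Surround row, then resizes the pool, passing the parent's first tag to new spawns as HostTag.
; Pooled actors are spaced evenly around the circle and attached, so RotatingMovement carries them.
; Shrinking only drops array entries without destroying those actors.
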(event `self.ReceiveBeginPlay`
  (`self.Init_SurroundPool`))

(fn `Create_Surrounds`
  (params (Surround_RowName :type Name) (Surround_Amount :type Integer))
  (bind _rotation_radius (`self.Rotation_Radius`))
  (bind (_returnvalue_x _returnvalue_y _returnvalue_z) (`KismetMathLibrary.BreakVector` (`self.K2_GetActorLocation` (`self.GetParentActor`))))
  (`self.Setup_Surrounds` Surround_RowName Surround_Amount)
  (`self.Update Surround Pool` Surround_Amount) ; 不论传入的数量是增是减,\n都将Pool设置为满足数量的情况
  (set `RotatingMovementComponent.RotationRate` (`KismetMathLibrary.MakeRotator` 0.0 0.0 (`self.Rotation_Rate`)) (`self.RotatingMovement`))
  (for (_array_element _array_index) (`self.Surround_Pool`)
    (bind _returnvalue (* _array_index (/ (* (`KismetMathLibrary.GetPI`) 2.0) (`self.Surround_Amount`))))
    (`self.K2_SetActorLocation` _array_element (`KismetMathLibrary.MakeVector_NetQuantize` (+ (* (`KismetMathLibrary.Cos` _returnvalue) _rotation_radius) _returnvalue_x) (+ (* _rotation_radius (`KismetMathLibrary.Sin` _returnvalue)) _returnvalue_y) _returnvalue_z) false true)
    (`self.K2_AttachToActor` _array_element self "None" "KeepWorld" "KeepRelative" "KeepRelative" true)))

(fn `Init_SurroundPool`
  (`KismetArrayLibrary.Array_Clear` (`self.Surround_Pool`)))

(fn `Setup_Surrounds`
  (params (Surround_RowName :type Name) (Surround_Amount :type Integer))
  (bind _output_get (set `self.Surround_RowName` Surround_RowName))
  (set `self.Surround_Amount` Surround_Amount)
  (bind _returnvalue (`|GetDataTableRow` "/Game/BluePrints/Objects/Surround/DT_Surround.DT_Surround" _output_get)
    (:`then`
      (bind ((`Surround_Sprite_11_233AB73C4B17292A61F46B93ECC496F9` _surround_sprite) (`DataAsset_5_F98685DA400D10DA89818991F0241283` _dataasset)) (break `/Game/BluePrints/Objects/Surround/S_Surround` _returnvalue))
      (set `self.Rotation_Radius` (`/Game/BluePrints/Objects/Surround/DataAssets/BP_DA_Surround.Surround_Rotation_Radius` _dataasset))
      (set `self.Rotation_Rate` (`/Game/BluePrints/Objects/Surround/DataAssets/BP_DA_Surround.Surround_Rotation_Rate` _dataasset))
      (return))))

(fn `Update Surround Pool`
  (params (Surround_Amount_New :type Integer))
  (locals (Local_HostTag :type Name) (Local_Surround_Amount_ToAdd :type Integer))
  (bind _local_surround_amount_toadd (`local.Local_Surround_Amount_ToAdd`))
  (bind _surround_pool (`self.Surround_Pool`))
  (bind _output_get (set `local.Local_Surround_Amount_ToAdd` (- Surround_Amount_New (`KismetArrayLibrary.Array_Length` (`self.Surround_Pool`)))))
  (if (> _output_get 0)
    (set `local.Local_HostTag` (`|GetArrayItem` (`Actor.Tags` (`self.GetParentActor`))))
    (for _ (range 1 (+ (`local.Local_Surround_Amount_ToAdd`) 1))
      (bind _returnvalue (`|SpawnActorFromClass` "/Game/BluePrints/Objects/Surround/BP_Surround.BP_Surround_C" (`KismetMathLibrary.MakeTransform` (0.0 0.0 500.0)) "AlwaysSpawn" "MultiplyWithRoot" null (`self.Surround_RowName`) (`local.Local_HostTag`) null))
      (`KismetArrayLibrary.Array_Add` (`self.Surround_Pool`) _returnvalue))
    (elif (< _local_surround_amount_toadd 0)
      (for _ (range (* _local_surround_amount_toadd -1))
        (`KismetArrayLibrary.Array_Remove` _surround_pool (`KismetArrayLibrary.Array_LastIndex` _surround_pool))
        (`KismetSystemLibrary.PrintString` "Hello" true true (struct :`G` 0.66 :`B` 1.0 :`A` 1.0) 22220.0))
      (else
        (return)))))

(fn `UserConstructionScript`)