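; Data asset Blueprint holding the stats of a Surround object: name, damage, knockback, flipbook playback, orbit motion, and sprite and collision sizes.
; SurroundInitDataAsset looks up a named row in DT_Surround_Init_DA and, when found, passes its fields to SurroundSetAll.
; SurroundSetAll copies every value into the asset's variables, so the DataTable seeds the asset's values.
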(fn `Surround_init_DataAsset`
  (params (Surround_RowName :type Name))
  (bind _returnvalue (`|GetDataTableRow` "/Game/BluePrints/Objects/Surround/DataAssets/Init_DA/DT_Surround_Init_DA.DT_Surround_Init_DA" Surround_RowName)
    (:`then`
      (bind (_surround_name _damage_value _knockback_value _flipbook_playrate _surround_rotation_radius _surround_rotation_rate _sprite_size _collision_size) (break `/Game/BluePrints/Objects/Surround/DataAssets/Init_DA/S_Surround_Init_DA` _returnvalue))
      (`self.Surround_Set_All` _surround_name _damage_value _knockback_value _flipbook_playrate _surround_rotation_radius _surround_rotation_rate _sprite_size _collision_size)
      (return))))

(fn `Surround_Set_All`
  (params (Surround_Name :type Text) (Damage_Value :type Integer) (Knockback_Value :type Integer) (Flipbook_PlayRate :type "Float (double-precision)") (Surround_Rotation_Radius :type "Float (double-precision)") (Surround_Rotation_Rate :type "Float (double-precision)") (Sprite_Size :type "Vector Structure") (Collision_Size :type "Vector Structure"))
  (set `self.Surround_Name` Surround_Name)
  (set `self.Damage_Value` Damage_Value)
  (set `self.Knockback_Value` Knockback_Value)
  (set `self.Flipbook_PlayRate` Flipbook_PlayRate)
  (set `self.Surround_Rotation_Radius` Surround_Rotation_Radius)
  (set `self.Surround_Rotation_Rate` Surround_Rotation_Rate)
  (set `self.Sprite_Size` Sprite_Size)
  (set `self.Collision_Size` Collision_Size)
  (return))