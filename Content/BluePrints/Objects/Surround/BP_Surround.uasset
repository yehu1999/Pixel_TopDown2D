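; BP_Surround is a data-driven flipbook object that deals damage and knockback to entities touching its sphere.
; On construction, its row in DT_Surround supplies the flipbook and a data asset that sets play rate, sprite and collision scale, and hit values.
; Overlaps damage BPI_Entity actors lacking the HostTag, sparing the host side.
; Tick pins world rotation to zero, and GetObjectInfo reports its object type and row name.
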(event `self.ReceiveBeginPlay`)

(event `self.ReceiveTick`
  (params (DeltaSeconds :type "Float (single-precision)"))
  (`self.K2_SetActorRotation` (struct)))

(event `self.Sphere.OnComponentBeginOverlap`
  (params (OverlappedComponent :type "PrimitiveComponent Object Reference") (OtherActor :type "Actor Object Reference") (OtherComp :type "PrimitiveComponent Object Reference") (OtherBodyIndex :type Integer) (bFromSweep :type Boolean) (SweepResult :type "HitResult Structure (by ref)"))
  (bind _data_asset (`self.Data Asset`))
  (if (and (not (`self.ActorHasTag` OtherActor (`self.Host_Tag`))) (`KismetSystemLibrary.DoesImplementInterface` OtherActor "/Game/Interfaces/BPI_Entity.BPI_Entity_C"))
    (message `/Game/Interfaces/BPI_Entity.Take Damage` OtherActor (`/Game/BluePrints/Objects/Surround/DataAssets/BP_DA_Surround.Damage_Value` _data_asset) self (`/Game/BluePrints/Objects/Surround/DataAssets/BP_DA_Surround.Knockback_Value` _data_asset))))

(fn `Get_Object_Info`
  (returns (Object_Type :type "/Game/BluePrints/Objects/E_ObjectType Enum") (Object_RowName :type Name))
  (return "NewEnumerator4" (`self.Surround_Row_Name`)))

(fn `Surround_Setup_Data`
  (params (Surround_Row_Name :type Name))
  (bind _output_get (set `self.Surround_Row_Name` Surround_Row_Name))
  (bind _returnvalue (`|GetDataTableRow` "/Game/BluePrints/Objects/Surround/DT_Surround.DT_Surround" _output_get)
    (:`then`
      (bind ((`Sprite_Flipbook_4_BFD740D84A92FC73E1FA3BB3AF08C751` _sprite_flipbook) (`Surround_Sprite_11_233AB73C4B17292A61F46B93ECC496F9` _surround_sprite) (`DataAsset_5_F98685DA400D10DA89818991F0241283` _dataasset)) (break `/Game/BluePrints/Objects/Surround/S_Surround` _returnvalue))
      (`PaperFlipbookComponent.SetFlipbook` (`self.PaperFlipbook`) _sprite_flipbook)
      (bind _output_get_2 (set `self.Data Asset` _dataasset))
      (`PaperFlipbookComponent.SetPlayRate` (`self.PaperFlipbook`) (`/Game/BluePrints/Objects/Surround/DataAssets/BP_DA_Surround.Flipbook_PlayRate` _output_get_2))
      (`SceneComponent.SetWorldScale3D` (`self.PaperFlipbook`) (`/Game/BluePrints/Objects/Surround/DataAssets/BP_DA_Surround.Sprite_Size` _output_get_2))
      (`SceneComponent.SetWorldScale3D` (`self.Sphere`) (`/Game/BluePrints/Objects/Surround/DataAssets/BP_DA_Surround.Collision_Size` _output_get_2)))))

(fn `UserConstructionScript`
  (`self.Surround_Setup_Data` (`self.Surround_Row_Name`)))