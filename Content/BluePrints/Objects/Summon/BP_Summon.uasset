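; BP_Summon is a pooled, data-driven summoned projectile that damages entities it overlaps.
; GetUp loads flipbook, speed, scale and damage data from DT_Summon, enables collision and starts the lifetime timer.
; Each BPI_Entity is hit once per activation, with caster magic power boosting damage and knockback, or dividing them with clamps against CallerTag actors.
; GoToSleep disables it, clears hits, parks it far away and removes it from the awake pool.
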(event `self.ReceiveBeginPlay`)

(event `self.ReceiveTick`
  (params (DeltaSeconds :type "Float (single-precision)")))

(event `self.Sphere.OnComponentBeginOverlap`
  (params (OverlappedComponent :type "PrimitiveComponent Object Reference") (OtherActor :type "Actor Object Reference") (OtherComp :type "PrimitiveComponent Object Reference") (OtherBodyIndex :type Integer) (bFromSweep :type Boolean) (SweepResult :type "HitResult Structure (by ref)"))
  (bind _data_asset (`self.Data Asset`))
  (bind _data_asset_2 (`self.Data Asset`))
  (switch `/Game/Instance/E_ActorPoolState` (`self.Summon_State`)
    (:`NewEnumerator0`
      (if (`KismetSystemLibrary.DoesImplementInterface` OtherActor "/Game/Interfaces/BPI_Entity.BPI_Entity_C")
        (if (not (`KismetArrayLibrary.Array_Contains` (`self.HItActor`) OtherActor))
          (`KismetArrayLibrary.Array_AddUnique` (`self.HItActor`) OtherActor)
          (if (not (`self.ActorHasTag` OtherActor (`self.Caller_Tag`)))
            (message `/Game/Interfaces/BPI_Entity.Take Damage` OtherActor (+ (`/Game/BluePrints/Objects/Summon/DataAsset/BP_DA_Summon.Damage_Value` _data_asset_2) (`self.Caller_MagicPower`)) self (+ (`/Game/BluePrints/Objects/Summon/DataAsset/BP_DA_Summon.Knockback_Value` _data_asset_2) (`self.Caller_MagicPower`)))
            (else
              (message `/Game/Interfaces/BPI_Entity.Take Damage` OtherActor (`KismetMathLibrary.Clamp` (/ (`/Game/BluePrints/Objects/Summon/DataAsset/BP_DA_Summon.Damage_Value` _data_asset) (`self.Caller_MagicPower`)) 5 15) self (`KismetMathLibrary.Clamp` (/ (`/Game/BluePrints/Objects/Summon/DataAsset/BP_DA_Summon.Knockback_Value` _data_asset) (`self.Caller_MagicPower`)) 20 999)))))))))

(fn `Get_Object_Info`
  (returns (Object_Type :type "/Game/BluePrints/Objects/E_ObjectType Enum") (Object_RowName :type Name))
  (return "NewEnumerator3" (`self.Summon_Row_Name`)))

(fn `Summon_GetUp`
  (params (Summon_RowName :type Name) (Launch_Direction :type "Vector Structure") (Caller_Tag :type Name) (Caller_MagicPower :type Integer))
  (bind _awake_time (`/Game/BluePrints/Objects/Summon/DataAsset/BP_DA_Summon.Awake_Time` (`self.Data Asset`)))
  (set `self.Caller_MagicPower` Caller_MagicPower)
  (`self.Summon_Setup_Data` Summon_RowName Launch_Direction Caller_Tag)
  (`self.Summon_Setup_Setting`)
  (set `self.Summon_State` "NewEnumerator0")
  (if (>= _awake_time 0.0)
    (`KismetSystemLibrary.K2_ClearAndInvalidateTimerHandle` (`self.Timer_AwakeTime`))
    (bind _returnvalue (`KismetSystemLibrary.K2_SetTimer` null "Summon_GoTo_Sleep" _awake_time))
    (set `self.Timer_AwakeTime` _returnvalue)))

(fn `Summon_GoTo_Sleep`
  (`self.Summon_Setdown_Setting`)
  (set `self.Summon_State` "NewEnumerator1")
  (`self.K2_SetActorLocation` (0.0 0.0 50000.0))
  (`KismetArrayLibrary.Array_RemoveItem` (`/Game/Instance/BP_ActorPool.Summon_Pool_Awake` (`/Game/Instance/BP_GameInstance_Pixels.ActorPool` (`/Game/Instance/Public/FL_Public.Get_GameInstance_Pixels`))) self)
  (`KismetSystemLibrary.K2_ClearAndInvalidateTimerHandle` (`self.Timer_AwakeTime`)))

(fn `Summon_Setdown_Setting`
  (`MovementComponent.StopMovementImmediately` (`self.ProjectileMovement`))
  (`ActorComponent.SetComponentTickEnabled` (`self.PaperFlipbook`) false)
  (`self.SetActorTickEnabled` false)
  (`PrimitiveComponent.SetCollisionEnabled` (`self.Sphere`) "NoCollision")
  (`KismetArrayLibrary.Array_Clear` (`self.HItActor`)))

(fn `Summon_Setup_Data`
  (params (`Projectile Row Name` :type Name) (LanuchDirection :type "Vector Structure") (CallerTag :type Name))
  (bind _output_get (set `self.Summon_Row_Name` `Projectile Row Name`))
  (bind _returnvalue (`|GetDataTableRow` "/Game/BluePrints/Objects/Summon/DT_Summon.DT_Summon" _output_get)
    (:`then`
      (bind (_sprite_flipbook _summon_sprite _summon_icon _dataasset) (break `/Game/BluePrints/Objects/Summon/S_Summon` _returnvalue))
      (`PaperFlipbookComponent.SetFlipbook` (`self.PaperFlipbook`) _sprite_flipbook)
      (bind _output_get_2 (set `self.Data Asset` _dataasset))
      (set `MovementComponent.Velocity` (* LanuchDirection (`/Game/BluePrints/Objects/Summon/DataAsset/BP_DA_Summon.Speed` _output_get_2)) (`self.ProjectileMovement`))
      (`PaperFlipbookComponent.SetPlayRate` (`self.PaperFlipbook`) (`/Game/BluePrints/Objects/Summon/DataAsset/BP_DA_Summon.Flipbook_PlayRate` _output_get_2))
      (`SceneComponent.SetWorldScale3D` (`self.PaperFlipbook`) (`/Game/BluePrints/Objects/Summon/DataAsset/BP_DA_Summon.Sprite_Size` _output_get_2))
      (`SceneComponent.SetWorldScale3D` (`self.Sphere`) (`/Game/BluePrints/Objects/Summon/DataAsset/BP_DA_Summon.Collision_Size` _output_get_2))
      (set `self.Caller_Tag` CallerTag))))

(fn `Summon_Setup_Setting`
  (`ActorComponent.SetComponentTickEnabled` (`self.PaperFlipbook`) true)
  (`self.SetActorTickEnabled` true)
  (`PrimitiveComponent.SetCollisionEnabled` (`self.Sphere`) "QueryOnly"))

(fn `UserConstructionScript`
  (`self.Summon_Setup_Data` (`self.Summon_Row_Name`) (`self.GetActorForwardVector`) (`self.Caller_Tag`)))