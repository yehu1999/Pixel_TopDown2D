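; BP_DA_Summon is a data asset Blueprint holding a summon's stats: name, combat effects, movement, timing, and flipbook and size settings.
; InitDataAsset looks up a row in DT_Summon_DA_Init by name and, if found, passes its fields to AssetSetAll, which copies them into the asset's variables.
; A separate setter overrides the damage value alone.
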(fn `Asset_Set_All`
  (params (Summon_Name :type Text) (Damage_Value :type Integer) (Knockback_Value :type Integer) (SpecialEffect_Type :type "/Game/BluePrints/Objects/Summon/DataAsset/E_Summon_SpecialEffect Enum" :default "NewEnumerator0") (SpecialEffect_Value :type "Float (double-precision)") (Speed :type "Float (double-precision)") (Flipbook_PlayRate :type "Float (double-precision)") (Awake_Time :type "Float (double-precision)") (Sprite_Size :type "Vector Structure") (Collision_Size :type "Vector Structure"))
  (set `self.Summon_Name` Summon_Name)
  (set `self.Damage_Value` Damage_Value)
  (set `self.Knockback_Value` Knockback_Value)
  (set `self.SpecialEffect_Type` SpecialEffect_Type)
  (set `self.SpecialEffect_Value` SpecialEffect_Value)
  (set `self.Speed` Speed)
  (set `self.Flipbook_PlayRate` Flipbook_PlayRate)
  (set `self.Awake_Time` Awake_Time)
  (set `self.Sprite_Size` Sprite_Size)
  (set `self.Collision_Size` Collision_Size)
  (return))

(fn `Init_DataAsset`
  (params (Projectile_RowName :type Name))
  (bind _returnvalue (`|GetDataTableRow` "/Game/BluePrints/Objects/Summon/DataAsset/Init_DA/DT_Summon_DA_Init.DT_Summon_DA_Init" Projectile_RowName)
    (:`then`
      (bind (_summon_name _damage_value _knockback_value _specialeffect_type _specialeffect_value _speed _flipbook_playrate _awake_time _sprite_size _collision_size) (break `/Game/BluePrints/Objects/Summon/DataAsset/Init_DA/S_Summon_DA_Init` _returnvalue))
      (`self.Asset_Set_All` _summon_name _damage_value _knockback_value _specialeffect_type _specialeffect_value _speed _flipbook_playrate _awake_time _sprite_size _collision_size)
      (return))))

(fn `Set_Damage_Value`
  (params (Damage_Value :type Integer))
  (set `self.Damage_Value` Damage_Value))