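; Data asset holding a projectile's tunable stats, such as damage, knockback, speed, sprite and collision size, and break and penetration behavior.
; InitDataAsset looks up a row by name in DT_Projectile_DA_Init and copies every field into the asset through AssetSetAll.
; Individual setters allow damage, knockback, sprite size and collision size to be changed separately.
; A missing row leaves the values unchanged.
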(fn `Asset_Set_All`
  (params (Projectile_Name :type Text) (Damage_Value :type Integer) (Knockback_Value :type Integer) (Speed :type "Float (double-precision)") (Flipbook_PlayRate :type "Float (double-precision)") (Awake_Time :type "Float (double-precision)") (Sprite_Size :type "Vector Structure") (Collision_Size :type "Vector Structure") (`Is Can Break` :type Boolean) (Scale_Break :type "Float (double-precision)") (`Break Time` :type "Float (double-precision)") (`Is Can Penetrate` :type Boolean))
  (set `self.Projectile_Name` Projectile_Name)
  (set `self.Damage_Value` Damage_Value)
  (set `self.Knockback_Value` Knockback_Value)
  (set `self.Speed` Speed)
  (set `self.Flipbook_PlayRate` Flipbook_PlayRate)
  (set `self.Awake_Time` Awake_Time)
  (set `self.Sprite_Size` Sprite_Size)
  (set `self.Collision_Size` Collision_Size)
  (set `self.Is Can Break` `Is Can Break`)
  (set `self.Scale_Break` Scale_Break)
  (set `self.Break Time` `Break Time`)
  (set `self.Is Can Penetrate` `Is Can Penetrate`)
  (return))

(fn `Asset_Set_Collision_Size`
  (params (New_Collision_Size :type "Vector Structure"))
  (set `self.Collision_Size` New_Collision_Size))

(fn `Asset_Set_Damage_Value`
  (params (New_Damage_Value :type Integer))
  (set `self.Damage_Value` New_Damage_Value))

(fn `Asset_Set_Knockback_Value`
  (params (NewKnockback_Value :type Integer))
  (set `self.Knockback_Value` NewKnockback_Value))

(fn `Asset_Set_Sprite_Size`
  (params (New_Sprite_Size :type "Vector Structure"))
  (set `self.Sprite_Size` New_Sprite_Size))

(fn `Init_DataAsset`
  (params (Projectile_RowName :type Name))
  (bind _returnvalue (`|GetDataTableRow` "/Game/BluePrints/Objects/Projectile/DataAssets/Init_DA/DT_Projectile_DA_Init.DT_Projectile_DA_Init" Projectile_RowName)
    (:`then`
      (bind (_projectile_name _damage_value _knockback_value _speed _flipbook_playrate _awake_time _sprite_size _collision_size _is_canbreak _scale_break _break_time _is_canpenetrate) (break `/Game/BluePrints/Objects/Projectile/DataAssets/Init_DA/S_Projectile_DA_Init` _returnvalue))
      (`self.Asset_Set_All` _projectile_name _damage_value _knockback_value _speed _flipbook_playrate _awake_time _sprite_size _collision_size _is_canbreak _scale_break _break_time _is_canpenetrate)
      (return))))