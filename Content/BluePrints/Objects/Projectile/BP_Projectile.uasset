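; Pooled 2D projectile that damages and knocks back BPI_Entity actors, skipping those with the shooter's tag and repeat hits.
; ProjectileGetUp wakes it, applying flipbook, speed and size from a DT_Projectile row and its DataAsset, and starting a lifetime timer.
; On hit or timeout it breaks with an enlarged sphere and flipbook, penetrates briefly, or sleeps.
; Sleeping disables tick and collision, parks it out of view and removes it from the awake pool.
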(event `self.ReceiveBeginPlay`)

(event `self.Sphere.OnComponentBeginOverlap`
  (params (OverlappedComponent :type "PrimitiveComponent Object Reference") (OtherActor :type "Actor Object Reference") (OtherComp :type "PrimitiveComponent Object Reference") (OtherBodyIndex :type Integer) (bFromSweep :type Boolean) (SweepResult :type "HitResult Structure (by ref)"))
  (bind _data_asset (`self.Data Asset`))
  (switch `/Game/Instance/E_ActorPoolState` (`self.Projectile_State`)
    (:`NewEnumerator0`
      (if (and (not (`self.ActorHasTag` OtherActor (`self.Shooter_Tag`))) (`KismetSystemLibrary.DoesImplementInterface` OtherActor "/Game/Interfaces/BPI_Entity.BPI_Entity_C"))
        (if (not (`KismetArrayLibrary.Array_Contains` (`self.HItActor`) OtherActor))
          (`KismetArrayLibrary.Array_AddUnique` (`self.HItActor`) OtherActor)
          (message `/Game/Interfaces/BPI_Entity.Take Damage` OtherActor (+ (`/Game/BluePrints/Objects/Projectile/DataAssets/BP_DA_Projectile.Damage_Value` _data_asset) (`self.Shooter_Power`)) self (+ (`/Game/BluePrints/Objects/Projectile/DataAssets/BP_DA_Projectile.Knockback_Value` _data_asset) (`self.Shooter_Power`)))
          (`self.Break_OR_Penetrate_OR_Sleep`))))))

(event `Break_OR_Penetrate_OR_Sleep`
  (bind _data_asset (`self.Data Asset`))
  (bind _scale_break (`/Game/BluePrints/Objects/Projectile/DataAssets/BP_DA_Projectile.Scale_Break` _data_asset))
  (if (`/Game/BluePrints/Objects/Projectile/DataAssets/BP_DA_Projectile.Is Can Break` _data_asset)
    (`SceneComponent.SetWorldScale3D` (`self.Sphere`) (* (`/Game/BluePrints/Objects/Projectile/DataAssets/BP_DA_Projectile.Collision_Size` _data_asset) _scale_break))
    (bind _returnvalue (`|GetDataTableRow` "/Game/BluePrints/Objects/Projectile/DT_Projectile.DT_Projectile" (`self.Projectile Row Name`))
      (:`then`
        (`PaperFlipbookComponent.SetFlipbook` (`self.PaperFlipbook`) (`.Sprite_Flipbook_Break_16_F078C4594C6E7BCCD01BE693F21615CC` (break `/Game/BluePrints/Objects/Projectile/S_Projectile` _returnvalue)))
        (`SceneComponent.SetWorldScale3D` (`self.PaperFlipbook`) (* _scale_break (`/Game/BluePrints/Objects/Projectile/DataAssets/BP_DA_Projectile.Sprite_Size` _data_asset)))
        (`KismetSystemLibrary.Delay` 0.1)
        (`MovementComponent.StopMovementImmediately` (`self.ProjectileMovement`))
        (`KismetSystemLibrary.Delay` (`/Game/BluePrints/Objects/Projectile/DataAssets/BP_DA_Projectile.Break Time` _data_asset))
        (`self.Projectile_GoTo_Sleep`)))
    (else
      (if (`/Game/BluePrints/Objects/Projectile/DataAssets/BP_DA_Projectile.Is Can Penetrate` _data_asset)
        (`KismetSystemLibrary.Delay` 2.0))
      (`self.Projectile_GoTo_Sleep`))))

(fn `Get_Object_Info`
  (returns (Object_Type :type "/Game/BluePrints/Objects/E_ObjectType Enum") (Object_RowName :type Name))
  (return "NewEnumerator2" (`self.Projectile Row Name`)))

(fn `Projectile_GetUp`
  (params (Projectile_RowName :type Name) (Launch_Direction :type "Vector Structure") (Shooter_Tag :type Name) (Shooter_Power :type Integer))
  (bind _awake_time (`/Game/BluePrints/Objects/Projectile/DataAssets/BP_DA_Projectile.Awake_Time` (`self.Data Asset`)))
  (`|GetDataTableRow` "/Game/BluePrints/Objects/Projectile/DT_Projectile.DT_Projectile" Projectile_RowName ; 不存在的RowName就别唤醒了
    (:`then`
      (set `self.Shooter_Power` Shooter_Power)
      (`self.Projectile_Setup_Data` Projectile_RowName Launch_Direction Shooter_Tag)
      (`self.Projectile_Setup_Setting`)
      (set `self.Projectile_State` "NewEnumerator0")
      (if (>= _awake_time 0.0)
        (`KismetSystemLibrary.K2_ClearAndInvalidateTimerHandle` (`self.Timer_AwakeTime`))
        (bind _returnvalue (`KismetSystemLibrary.K2_SetTimer` null "Break_OR_Penetrate_OR_Sleep" _awake_time))
        (set `self.Timer_AwakeTime` _returnvalue)))))

(fn `Projectile_GoTo_Sleep`
  (`self.Projectile_Setdown_Setting`)
  (set `self.Projectile_State` "NewEnumerator1")
  (`self.K2_SetActorLocation` (0.0 0.0 50000.0))
  (`KismetArrayLibrary.Array_RemoveItem` (`/Game/Instance/BP_ActorPool.Character_ProjectilePool_Awake` (`/Game/Instance/BP_GameInstance_Pixels.ActorPool` (`/Game/Instance/Public/FL_Public.Get_GameInstance_Pixels`))) self)
  (`KismetSystemLibrary.K2_ClearAndInvalidateTimerHandle` (`self.Timer_AwakeTime`)))

(fn `Projectile_Setdown_Setting`
  (`MovementComponent.StopMovementImmediately` (`self.ProjectileMovement`))
  (`ActorComponent.SetComponentTickEnabled` (`self.PaperFlipbook`) false)
  (`self.SetActorTickEnabled` false)
  (`PrimitiveComponent.SetCollisionEnabled` (`self.Sphere`) "NoCollision")
  (`KismetArrayLibrary.Array_Clear` (`self.HItActor`)))

(fn `Projectile_Setup_Data`
  (params (`Projectile Row Name` :type Name) (LanuchDirection :type "Vector Structure") (ShooterTag :type Name))
  (bind _output_get (set `self.Projectile Row Name` `Projectile Row Name`))
  (bind _returnvalue (`|GetDataTableRow` "/Game/BluePrints/Objects/Projectile/DT_Projectile.DT_Projectile" _output_get)
    (:`then`
      (bind ((`Sprite_Flipbook_3_77E0DE2E4478E1BEDB5583976A496723` _sprite_flipbook) (`DataAsset_6_7622AA0049E3DCE69AE0F98C630F881B` _dataasset)) (break `/Game/BluePrints/Objects/Projectile/S_Projectile` _returnvalue))
      (`PaperFlipbookComponent.SetFlipbook` (`self.PaperFlipbook`) _sprite_flipbook)
      (bind _output_get_2 (set `self.Data Asset` _dataasset))
      (set `MovementComponent.Velocity` (* LanuchDirection (`/Game/BluePrints/Objects/Projectile/DataAssets/BP_DA_Projectile.Speed` _output_get_2)) (`self.ProjectileMovement`))
      (`PaperFlipbookComponent.SetPlayRate` (`self.PaperFlipbook`) (`/Game/BluePrints/Objects/Projectile/DataAssets/BP_DA_Projectile.Flipbook_PlayRate` _output_get_2))
      (`SceneComponent.SetWorldScale3D` (`self.PaperFlipbook`) (`/Game/BluePrints/Objects/Projectile/DataAssets/BP_DA_Projectile.Sprite_Size` _output_get_2))
      (`SceneComponent.SetWorldScale3D` (`self.Sphere`) (`/Game/BluePrints/Objects/Projectile/DataAssets/BP_DA_Projectile.Collision_Size` _output_get_2))
      (set `self.Shooter_Tag` ShooterTag))))

(fn `Projectile_Setup_Setting`
  (`ActorComponent.SetComponentTickEnabled` (`self.PaperFlipbook`) true)
  (`self.SetActorTickEnabled` true)
  (`PrimitiveComponent.SetCollisionEnabled` (`self.Sphere`) "QueryOnly"))

(fn `UserConstructionScript`
  (`self.Projectile_Setup_Data` (`self.Projectile Row Name`) (`self.GetActorForwardVector`))
  (set `self.Projectile_State` "NewEnumerator1") ; 放置在Map中的抛射物默认为Sleep
)