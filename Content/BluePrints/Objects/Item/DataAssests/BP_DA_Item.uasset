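; Item data asset Blueprint that holds an item's name, type, value, sprite size, collision size and awake time.
; InitDataAsset looks up a row by name in the DT_Item_DA_Init data table and, when found, passes its fields to AssetSetAll.
; AssetSetAll copies those values into the asset's variables, so the table drives each item's setup.
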(fn `Asset_Set_All`
  (params (ItemName :type Text) (Item_Type :type "/Game/BluePrints/Objects/Item/E_Item_type Enum" :default "NewEnumerator0") (Item_Value :type Integer) (Sprite_Size :type "Vector Structure") (Colllision_Size :type "Vector Structure") (Awake_Time :type "Float (double-precision)"))
  (set `self.ItemName` ItemName)
  (set `self.Item_Type` Item_Type)
  (set `self.Item_Value` Item_Value)
  (set `self.Sprite_Size` Sprite_Size)
  (set `self.Colllision_Size` Colllision_Size)
  (set `self.Awake_Time` Awake_Time)
  (return))

(fn `Init_DataAsset`
  (params (Item_RowName :type Name))
  (bind _returnvalue (`|GetDataTableRow` "/Game/BluePrints/Objects/Item/DataAssests/Init_DA/DT_Item_DA_Init.DT_Item_DA_Init" Item_RowName)
    (:`then`
      (bind (_item_name _item_type _item_value _sprite_size _collision_szie _awake_time) (break `/Game/BluePrints/Objects/Item/DataAssests/Init_DA/S_Item_DA_Init` _returnvalue))
      (`self.Asset_Set_All` _item_name _item_type _item_value _sprite_size _collision_szie _awake_time)
      (return))))