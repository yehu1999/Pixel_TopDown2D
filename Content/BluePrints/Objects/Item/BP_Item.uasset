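; Pooled pickup item with a Paper2D flipbook, configured by row name from DT_Item and its DataAsset.
; An overlapping actor that has learned the "Pickup" skill draws the item in through a timeline-driven VInterpTo, then receives its type and value.
; GetUp wakes it with an optional timed return; GoToSleep disables tick and collision and parks it high above the map.
; BeginPlay initializes every row's DataAsset, as the row may be unset then.
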(event `self.ReceiveBeginPlay`
  (`self.Item_Init_DataAsset_All` true))

(event `self.Sphere.OnComponentBeginOverlap`
  (params (OverlappedComponent :type "PrimitiveComponent Object Reference") (OtherActor :type "Actor Object Reference") (OtherComp :type "PrimitiveComponent Object Reference") (OtherBodyIndex :type Integer) (bFromSweep :type Boolean) (SweepResult :type "HitResult Structure (by ref)"))
  (bind (_skillrank _has_learn_thisskill) (message `/Game/Interfaces/BPI_Entity.Has Learned This Skill` OtherActor "Pickup"))
  (if _has_learn_thisskill
    (set `self.Interacting_Actor` OtherActor)
    (switch `/Game/BluePrints/Objects/Item/E_Item_type` (`/Game/BluePrints/Objects/Item/DataAssests/BP_DA_Item.Item_Type` (`self.Data Asset`))
      (:`NewEnumerator0`
        _)
      (:`NewEnumerator2`
        _)
      (:`NewEnumerator1`
        _)
      (:`NewEnumerator3`
        _))
    (`self.FlyTo_Pickuper`)))

(event `FlyTo_Pickuper`
  (bind _data_asset (`self.Data Asset`))
  (bind _item_type (`/Game/BluePrints/Objects/Item/DataAssests/BP_DA_Item.Item_Type` _data_asset))
  (`Timeline|TimeLine_FlyToPickuper` :!via `PlayFromStart`
    (:`Update`
      (`/Engine/EditorBlueprintResources/StandardMacros.IsValid` (`self.Interacting_Actor`)
        (:`Is Valid`
          (`self.K2_SetActorLocation` (`KismetMathLibrary.VInterpTo` (`self.K2_GetActorLocation`) (`self.K2_GetActorLocation` (`self.Interacting_Actor`)) (`GameplayStatics.GetWorldDeltaSeconds`) 8.0))
          (if (<= (`self.GetDistanceTo` (`self.Interacting_Actor`)) 15.0)
            (`TimelineComponent.Stop` (`self.TimeLine_FlyToPickuper`))
            (message `/Game/Interfaces/BPI_Entity.Take_Item` (`self.Interacting_Actor`) _item_type "None" (`/Game/BluePrints/Objects/Item/DataAssests/BP_DA_Item.Item_Value` _data_asset))
            (switch `/Game/BluePrints/Objects/Item/E_Item_type` _item_type
              (:`NewEnumerator0`
                (`GameplayStatics.PlaySound2D` "/Game/Audios/SFX/SoundCue_Item_Coins.SoundCue_Item_Coins" 1.0 1.0 0.0 null null))
              (:`NewEnumerator2`
                _)
              (:`NewEnumerator1`
                _)
              (:`NewEnumerator3`
                _))
            (`self.Item_GoTo_Sleep`)))
        (:`Is Not Valid`
          (`TimelineComponent.Stop` (`self.TimeLine_FlyToPickuper`)))))))

(fn `Get_Object_Info`
  (returns (Object_Type :type "/Game/BluePrints/Objects/E_ObjectType Enum") (Object_RowName :type Name))
  (return "NewEnumerator0" (`self.Item_RowName`)))

(fn `Item_GetUp`
  (params (Item_RowName :type Name))
  (bind _awake_time (`/Game/BluePrints/Objects/Item/DataAssests/BP_DA_Item.Awake_Time` (`self.Data Asset`)))
  (`self.Item_Setup_Data` Item_RowName)
  (`self.Item_Setup_Setting`)
  (set `self.Item_State` "NewEnumerator0")
  (if (> _awake_time 0.0)
    (`KismetSystemLibrary.K2_ClearAndInvalidateTimerHandle` (`self.Timer_AwakeTime`))
    (bind _returnvalue (`KismetSystemLibrary.K2_SetTimer` null "Item_GoTo_Sleep" _awake_time))
    (set `self.Timer_AwakeTime` _returnvalue)))

(fn `Item_GoTo_Sleep`
  (`self.Item_Setdown_Setting`)
  (set `self.Item_State` "NewEnumerator1")
  (`self.K2_SetActorLocation` (0.0 0.0 50000.0))
  (`KismetSystemLibrary.K2_ClearAndInvalidateTimerHandle` (`self.Timer_AwakeTime`)))

(fn `Item_Init_DataAsset_All`
  (params (Is_From_DT_DA_Init :type Boolean) (Is_From_Profile :type Boolean))
  (if Is_From_DT_DA_Init
    (bind _outrownames (`DataTableFunctionLibrary.GetDataTableRowNames` "/Game/BluePrints/Objects/Item/DT_Item.DT_Item")) ; 因为Item在游戏开始时并未设置具体RowName,\n所以初始化DA时需要将所有Item的DA都初始化，\n或许有更好的解决方案，但暂时先这样处理
    (for _array_element _outrownames
      (bind _returnvalue (`|GetDataTableRow` "/Game/BluePrints/Objects/Item/DT_Item.DT_Item" _array_element)
        (:`then`
          (`/Game/BluePrints/Objects/Item/DataAssests/BP_DA_Item.Init_DataAsset` (`.DataAsset_10_FA0939974D2C03647B035C9CDA4E2FD2` (break `/Game/BluePrints/Objects/Item/S_Item` _returnvalue)) _array_element))))
    (return)
    (else
      ;[1 1 1] TODO
      (if Is_From_Profile
        _))))

(fn `Item_Setdown_Setting`
  (`ActorComponent.SetComponentTickEnabled` (`self.PaperFlipbook`) false)
  (`self.SetActorTickEnabled` false)
  (`PrimitiveComponent.SetCollisionEnabled` (`self.Sphere`) "NoCollision")
  (set `self.Interacting_Actor` null))

(fn `Item_Setup_Data`
  (params (Item_RowName :type Name))
  (bind _output_get (set `self.Item_RowName` Item_RowName))
  (bind _returnvalue (`|GetDataTableRow` "/Game/BluePrints/Objects/Item/DT_Item.DT_Item" _output_get)
    (:`then`
      (bind (_item_spriteflipbook _item_sprite _item_icon _dataasset) (break `/Game/BluePrints/Objects/Item/S_Item` _returnvalue))
      (`PaperFlipbookComponent.SetFlipbook` (`self.PaperFlipbook`) _item_spriteflipbook)
      (bind _output_get_2 (set `self.Data Asset` _dataasset))
      (`SceneComponent.SetWorldScale3D` (`self.PaperFlipbook`) (`/Game/BluePrints/Objects/Item/DataAssests/BP_DA_Item.Sprite_Size` _output_get_2))
      (`SceneComponent.SetWorldScale3D` (`self.Sphere`) (`/Game/BluePrints/Objects/Item/DataAssests/BP_DA_Item.Colllision_Size` _output_get_2)))))

(fn `Item_Setup_Setting`
  (`ActorComponent.SetComponentTickEnabled` (`self.PaperFlipbook`) true)
  (`self.SetActorTickEnabled` true)
  (`PrimitiveComponent.SetCollisionEnabled` (`self.Sphere`) "QueryOnly"))

(fn `UserConstructionScript`
  (`self.Item_Setup_Data` (`self.Item_RowName`))
  (set `self.Item_State` "NewEnumerator0") ; 放置在Map中的Item默认为Awake
)