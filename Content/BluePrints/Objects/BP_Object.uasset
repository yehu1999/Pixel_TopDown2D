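; BP_Object is a poolable 2D sprite object whose look comes from an object type and row name.
; GetUp applies the sprite, enables tick and query collision, and starts a timeout that sends it to sleep.
; Sleep disables it and parks it far away on Z instead of destroying it.
; ObjectJump plays a timeline-driven sprite arc, mirrored horizontally according to which side of the character it is on.
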(event `ObjectJump`
  (if (`/Game/Instance/Public/FL_Public.Check_Is_A_At_B_Right` self (`/Game/Instance/Public/FL_Public.Get_Character`))
    (bind (_direction _x _y) (`Timeline|TimeLine_Crop_Jump` :!via `PlayFromStart`)
      (:`Update`
        (`SceneComponent.K2_SetRelativeLocation` (`self.PaperSprite_Object`) (`KismetMathLibrary.MakeVector` _x _y) false false)))
    (else
      (bind (_direction_2 _x_2 _y_2) (`Timeline|时间轴` :!via `PlayFromStart`)
        (:`Update`
          (`SceneComponent.K2_SetRelativeLocation` (`self.PaperSprite_Object`) (`KismetMathLibrary.MakeVector` (* _x_2 -1.0) _y_2) false false))))))

(fn `Get_Object_Info`
  (returns (Object_Type :type "/Game/BluePrints/Objects/E_ObjectType Enum") (Object_RowName :type Name))
  (return (`self.Object_Type`) (`self.Object_RowName`)))

(fn `Object_GetUp`
  (params (Object_Type :type "/Game/BluePrints/Objects/E_ObjectType Enum" :default "NewEnumerator6") (Object_RowName :type Name))
  (`self.Object_Setup_Data` Object_Type Object_RowName)
  (`self.Object_Setup_Setting`)
  (set `self.Object_State` "NewEnumerator0")
  (`KismetSystemLibrary.K2_ClearAndInvalidateTimerHandle` (`self.Timer_AwakeTime`))
  (bind _returnvalue (`KismetSystemLibrary.K2_SetTimer` null "Object_GoTo_Sleep" 120.0))
  (set `self.Timer_AwakeTime` _returnvalue))

(fn `Object_GoTo_Sleep`
  (`self.Object_Setdown_Setting`)
  (set `self.Object_State` "NewEnumerator1")
  (`self.K2_SetActorLocation` (0.0 0.0 50000.0))
  (`KismetSystemLibrary.K2_ClearAndInvalidateTimerHandle` (`self.Timer_AwakeTime`)))

(fn `Object_Setdown_Setting`
  (`ActorComponent.SetComponentTickEnabled` (`self.PaperSprite_Object`) false)
  (`self.SetActorTickEnabled` false)
  (`PrimitiveComponent.SetCollisionEnabled` (`self.PaperSprite_Object`) "NoCollision")
  (`SceneComponent.K2_SetRelativeLocation` (`self.PaperSprite_Object`) (0.0 0.0 0.0) false false))

(fn `Object_Setup_Data`
  (params (Object_Type :type "/Game/BluePrints/Objects/E_ObjectType Enum" :default "NewEnumerator6") (Object_RowName :type Name))
  (bind _output_get (set `self.Object_Type` Object_Type))
  (bind _output_get_2 (set `self.Object_RowName` Object_RowName))
  (bind _object_sprite (`/Game/Instance/Public/FL_Public.Break_Object` _output_get _output_get_2))
  (`PaperSpriteComponent.SetSprite` (`self.PaperSprite_Object`) _object_sprite))

(fn `Object_Setup_Setting`
  (`ActorComponent.SetComponentTickEnabled` (`self.PaperSprite_Object`) true)
  (`self.SetActorTickEnabled` true)
  (`PrimitiveComponent.SetCollisionEnabled` (`self.PaperSprite_Object`) "QueryOnly"))

(fn `UserConstructionScript`
  (`self.Object_Setup_Data` (`self.Object_Type`) (`self.Object_RowName`)))