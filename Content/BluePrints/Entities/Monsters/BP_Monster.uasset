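; Pooled 2D flipbook monster Character that fights the player, set up per DT_Monster row from a DataAsset of stats and skills.
; GetUp starts its behavior tree and optional lifetime timer; GoToSleep disables it and parks it out of sight for reuse.
; It attacks by body contact, directional weapon box, fanned pooled projectiles or speed-boosting rush, re-toggling collision to repeat hits.
; Damage triggers flash, numbers and weight-reduced knockback; death grants EXP and drops a coin.
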(event `self.ReceiveBeginPlay`
  ;[1 1 1] Begin/Tick
  (switch `/Game/BluePrints/Entities/Monsters/E_Monster_States` (`self.Monster_State`)))

(event `self.ReceiveTick`
  (params (DeltaSeconds :type "Float (single-precision)"))
  (bind _returnvalue (`self.GetVelocity`))
  ;[1 1 1] Begin/Tick
  (`|ExecutionSequence`
    (:`then_0`
      (`self.K2_SetActorRotation` (struct)) ; Keep Actor Rotation
      (if (not (== (`KismetMathLibrary.VSizeXY` _returnvalue) 0.0))
        (set `self.Direction` (`KismetMathLibrary.MakeVector2D` (.x _returnvalue) (.y _returnvalue))) ; ABP将根据Direction改变不同朝向的动画
        (`self.Monster_Update_BoxWeaponLocation`)))))

(event `Launch_Projectile`
  (bind _dataasset (`self.DataAsset`))
  ;[1 1 1] BehaviorTree
  ;;[1 1 1] Shoot
  (for _index (range (`/Game/BluePrints/Entities/Monsters/DataAssets/BP_DA_Monster.MultiShoot_Amount` (`self.DataAsset`)))
    (bind _sussess (`/Game/Instance/BP_ActorPool.Monster_Awake_A_Projectile` (`/Game/Instance/Public/FL_Public.Get_ActorPool`) (`/Game/BluePrints/Entities/Monsters/DataAssets/BP_DA_Monster.Projectile_RowName` _dataasset) (`self.K2_GetActorLocation`) (`self.Get_LanuchDirection` _index) "Monster" (`/Game/BluePrints/Entities/Monsters/DataAssets/BP_DA_Monster.Power` _dataasset)))
    (if _sussess
      (`GameplayStatics.PlaySound2D` "/Game/Audios/SFX/SoundCue_Character_Shoot.SoundCue_Character_Shoot" 0.5 1.0 0.0 null null))))

(event `Start_Rush`
  (bind _dataasset (`self.DataAsset`))
  ;[1 1 1] BehaviorTree
  ;;[1 1 1] Rush
  (set `/Game/BluePrints/Entities/Monsters/ABP_Monster.Is_Rushing` true (`/Game/Instance/Public/FL_Public.Get_ABP_Monster` self))
  (set `CharacterMovementComponent.MaxWalkSpeed` (* (`/Game/BluePrints/Entities/Monsters/DataAssets/BP_DA_Monster.Speed` _dataasset) 2.0) (`self.CharacterMovement`))
  (`KismetSystemLibrary.Delay` (`/Game/BluePrints/Entities/Monsters/DataAssets/BP_DA_Monster.Asset_Get_Skill_Duration` _dataasset "Rush"))
  (`self.Stop_Rush`))

(event `/Game/Interfaces/BPI_Entity.Take Damage`
  (params (Damage_Value :type Integer) (Attacker :type "Actor Object Reference") (Knockback_Value :type Integer))
  ;[1 1 1] 受伤/死亡
  (switch `/Game/BluePrints/Entities/Monsters/E_Monster_States` (`self.Monster_State`)
    (:`NewEnumerator0`
      (`self.FX_TakeDamage` Damage_Value Attacker Knockback_Value)
      (bind _output_get (set `self.HP` (- (`self.HP`) Damage_Value)))
      (if (<= _output_get 0)
        (message `/Game/Interfaces/BPI_Entity.Take_Item` (`GameplayStatics.GetPlayerPawn` 0) "NewEnumerator1" "None" (`/Game/BluePrints/Entities/Monsters/DataAssets/BP_DA_Monster.EXP_Base` (`self.DataAsset`)))
        (`self.Die`)))))

(event `Stop_Rush`
  ;[1 1 1] BehaviorTree
  ;;[1 1 1] Rush
  (set `/Game/BluePrints/Entities/Monsters/ABP_Monster.Is_Rushing` false (`/Game/Instance/Public/FL_Public.Get_ABP_Monster` self))
  (set `CharacterMovementComponent.MaxWalkSpeed` (`/Game/BluePrints/Entities/Monsters/DataAssets/BP_DA_Monster.Speed` (`self.DataAsset`)) (`self.CharacterMovement`)))

(event `FX_TakeDamage`
  (params (Damage_Value :type Integer) (Attacker :type "Actor Object Reference") (Konckback_Value :type Integer))
  ;[1 1 1] 受伤/死亡
  (`PaperFlipbookComponent.SetSpriteColor` (`self.Sprite`) (struct :`R` 0.5 :`A` 1.0))
  (`GameplayStatics.PlaySound2D` "/Game/Audios/SFX/SoundCue_Monster_TakeDamage.SoundCue_Monster_TakeDamage" 1.0 1.0 0.0 null null)
  (`self.Monster_Spawn Damage Number` Damage_Value)
  (`self.Monster_KnockBack` Attacker Konckback_Value)
  (`KismetSystemLibrary.Delay` 0.3)
  (`PaperFlipbookComponent.SetSpriteColor` (`self.Sprite`) (struct :`R` 1.0 :`G` 1.0 :`B` 1.0 :`A` 1.0)))

(event `Die`
  ;[1 1 1] 受伤/死亡
  (`GameplayStatics.PlaySound2D` "/Game/Audios/SFX/SoundCue_Monster_Die.SoundCue_Monster_Die" 1.0 1.0 0.0 null null)
  (`KismetSystemLibrary.K2_ClearAndInvalidateTimerHandle` (`self.Timer_AIMove`))
  (set `self.Monster_State` "NewEnumerator2")
  (`self.Monster_Drop_Items`)
  (set `/Game/BluePrints/Entities/Monsters/ABP_Monster.Is_Monster_Die` true (`/Game/Instance/Public/FL_Public.Get_ABP_Monster` self))
  (`/Engine/EditorBlueprintResources/StandardMacros.IncrementInt` (`/Game/BluePrints/Entities/Characters/BP_Character.KillNum` (`/Game/Instance/Public/FL_Public.Get_Character`))
    (:`  `
      (`KismetSystemLibrary.Delay` 0.8)
      (`self.Monster_GoTo_Sleep`))))

(event `self.Sphere_Body.OnComponentBeginOverlap`
  (params (OverlappedComponent :type "PrimitiveComponent Object Reference") (OtherActor :type "Actor Object Reference") (OtherComp :type "PrimitiveComponent Object Reference") (OtherBodyIndex :type Integer) (bFromSweep :type Boolean) (SweepResult :type "HitResult Structure (by ref)"))
  (bind _dataasset (`self.DataAsset`))
  ;[1 1 1] Overlap
  ;;[1 1 1] BodyOverlap/BodyAttack
  (if (`.Has_Learned_ThisSkill` (`/Game/BluePrints/Entities/Monsters/DataAssets/BP_DA_Monster.Asset Check This Skill` (`self.DataAsset`) "Attack_Body"))
    (switch `/Game/BluePrints/Entities/Monsters/E_Monster_States` (`self.Monster_State`)
      (:`NewEnumerator0`
        (if (and (not (`self.ActorHasTag` OtherActor "Monster")) (`KismetSystemLibrary.DoesImplementInterface` OtherActor "/Game/Interfaces/BPI_Entity.BPI_Entity_C"))
          (message `/Game/Interfaces/BPI_Entity.Take Damage` OtherActor (`/Game/BluePrints/Entities/Monsters/DataAssets/BP_DA_Monster.Damage_Value` _dataasset) self (`/Game/BluePrints/Entities/Monsters/DataAssets/BP_DA_Monster.KnockValue_Value` _dataasset))
          (`PrimitiveComponent.SetCollisionEnabled` (`self.Sphere_Body`) "NoCollision")
          (`KismetSystemLibrary.Delay` (`/Game/BluePrints/Entities/Monsters/DataAssets/BP_DA_Monster.Asset_Get_Skill_CycleTime` (`self.DataAsset`) "Attack_Body")) ; 强制重新检测
          (`PrimitiveComponent.SetCollisionEnabled` (`self.Sphere_Body`) "QueryOnly"))))))

(event `self.Box_Weapon.OnComponentBeginOverlap`
  (params (OverlappedComponent :type "PrimitiveComponent Object Reference") (OtherActor :type "Actor Object Reference") (OtherComp :type "PrimitiveComponent Object Reference") (OtherBodyIndex :type Integer) (bFromSweep :type Boolean) (SweepResult :type "HitResult Structure (by ref)"))
  (bind _dataasset (`self.DataAsset`))
  ;[1 1 1] Overlap
  ;;[1 1 1] WeaponOverlap/WeaponAttack
  (if (`.Has_Learned_ThisSkill` (`/Game/BluePrints/Entities/Monsters/DataAssets/BP_DA_Monster.Asset Check This Skill` (`self.DataAsset`) "Attack_Weapon"))
    (switch `/Game/BluePrints/Entities/Monsters/E_Monster_States` (`self.Monster_State`)
      (:`NewEnumerator0`
        (if (and (not (`self.ActorHasTag` OtherActor "Monster")) (`KismetSystemLibrary.DoesImplementInterface` OtherActor "/Game/Interfaces/BPI_Entity.BPI_Entity_C"))
          (bind _target_attack_weapon (`self.Target_Attack_Weapon`)
            (:`then`
              (if (== OtherActor _target_attack_weapon)
                (set `self.Target_Attack_Weapon` null) ; 重置目标
                (message `/Game/Interfaces/BPI_Entity.Take Damage` OtherActor (`/Game/BluePrints/Entities/Monsters/DataAssets/BP_DA_Monster.Damage_Value` _dataasset) self (`/Game/BluePrints/Entities/Monsters/DataAssets/BP_DA_Monster.KnockValue_Value` _dataasset))
                (`PrimitiveComponent.SetCollisionEnabled` (`self.Box_Weapon`) "NoCollision")
                (`KismetSystemLibrary.Delay` (`/Game/BluePrints/Entities/Monsters/DataAssets/BP_DA_Monster.Asset_Get_Skill_CycleTime` (`self.DataAsset`) "Attack_Weapon")) ; 强制重新检测
                (`PrimitiveComponent.SetCollisionEnabled` (`self.Box_Weapon`) "QueryOnly")
                (else
                  (set `self.Target_Attack_Weapon` OtherActor :!label _label)
                  (`self.Attack_Weapon`))))
            (:`else`
              (goto _label))))))))

(event `Attack_Weapon`
  (bind _returnvalue (/ (`/Game/BluePrints/Entities/Monsters/DataAssets/BP_DA_Monster.Asset_Get_Skill_Duration` (`self.DataAsset`) "Attack_Weapon") 2.0))
  ;[1 1 1] Overlap
  ;;[1 1 1] WeaponOverlap/WeaponAttack
  (set `/Game/BluePrints/Entities/Monsters/ABP_Monster.Is_Attacking` true (`/Game/Instance/Public/FL_Public.Get_ABP_Monster` self))
  (`PrimitiveComponent.SetCollisionEnabled` (`self.Box_Weapon`) "NoCollision")
  (`KismetSystemLibrary.Delay` _returnvalue) ; 强制重新检测
  (`PrimitiveComponent.SetCollisionEnabled` (`self.Box_Weapon`) "QueryOnly")
  (set `/Game/BluePrints/Entities/Monsters/ABP_Monster.Is_Attacking` false (`/Game/Instance/Public/FL_Public.Get_ABP_Monster` self))
  (`KismetSystemLibrary.Delay` _returnvalue) ; 攻击结束重置目标
  (set `self.Target_Attack_Weapon` null))

(fn `Get_Is_Alive`
  (returns (Is_Alive :type Boolean))
  (if (> (`self.HP`) 0)
    (return true)
    (else
      (return false))))

(fn `Get_LanuchDirection`
  (params (Launch_Index :type Integer))
  (returns (ReturnValue :type "Vector Structure"))
  (locals (Local_DeltaAngle :type "Float (double-precision)"))
  (bind _returnvalue (`KismetMathLibrary.FCeil` (/ Launch_Index 2)))
  (bind (_returnvalue_roll _returnvalue_pitch _returnvalue_yaw) (`KismetMathLibrary.BreakRotator` (`KismetMathLibrary.FindLookAtRotation` (`self.K2_GetActorLocation`) (`self.K2_GetActorLocation` (`/Game/Instance/Public/FL_Public.Get_Character`)))))
  (`|ExecutionSequence`
    (:`then_0`
      (if (`KismetMathLibrary.Conv_IntToBool` (mod Launch_Index 2))
        (set `local.Local_DeltaAngle` (* _returnvalue -12))
        (else
          (set `local.Local_DeltaAngle` (* _returnvalue 12)))))
    (:`then_1`
      (return (`KismetMathLibrary.Normal` (`KismetMathLibrary.Conv_RotatorToVector` (`KismetMathLibrary.MakeRotator` 0.0 0.0 (+ _returnvalue_yaw (`local.Local_DeltaAngle`)))))))))

(fn `Has Learned This Skill`
  (params (SkillTag :type Name))
  (returns (SkillRank :type Integer) (Has_Learn_ThisSkill :type Boolean))
  (bind (_skill_rank _has_learned_thisskill) (`/Game/BluePrints/Entities/Monsters/DataAssets/BP_DA_Monster.Asset Check This Skill` (`self.DataAsset`) SkillTag))
  (return _skill_rank _has_learned_thisskill))

(fn `Monster_Drop_Items`
  (`/Game/Instance/BP_ActorPool.Awake_A_Item` (`/Game/Instance/BP_GameInstance_Pixels.ActorPool` (`/Game/Instance/Public/FL_Public.Get_GameInstance_Pixels`)) "Item_Coin" (`KismetMathLibrary.MakeVector` (.x (`self.K2_GetActorLocation`)) (.y (`self.K2_GetActorLocation`)) 10.0)))

(fn `Monster_GetUp`
  (params (Monster_RowName :type Name))
  (bind _lifetime (`/Game/BluePrints/Entities/Monsters/DataAssets/BP_DA_Monster.LifeTime` (`self.DataAsset`)))
  (`self.Monster_Setup_Data` Monster_RowName)
  (`self.Monster_Setup_Setting`)
  (set `self.Monster_State` "NewEnumerator0")
  (`AIController.RunBehaviorTree` (`AIBlueprintHelperLibrary.GetAIController` self) "/Game/BluePrints/Entities/Monsters/AI/BT_Monster.BT_Monster")
  (`/Game/BluePrints/Entities/Monsters/AI/AIC_Monster.Start_BehaviorTree` (`/Game/Instance/Public/FL_Public.Get_AIC_Monster` self))
  (`|ExecutionSequence`
    (:`then_0`
      (if (>= _lifetime 0.0)
        (`KismetSystemLibrary.K2_ClearAndInvalidateTimerHandle` (`self.Timer_LifeTime`))
        (bind _returnvalue (`KismetSystemLibrary.K2_SetTimer` null "Monster_GoTo_Sleep" _lifetime))
        (set `self.Timer_LifeTime` _returnvalue)))))

(fn `Monster_GoTo_Sleep`
  (`self.Monster_Setdown_Setting`)
  (set `self.Monster_State` "NewEnumerator1")
  (`self.K2_SetActorLocation` (0.0 0.0 50000.0))
  (`KismetArrayLibrary.Array_RemoveItem` (`/Game/Instance/BP_ActorPool.MonsterPool_Awake` (`/Game/Instance/BP_GameInstance_Pixels.ActorPool` (`/Game/Instance/Public/FL_Public.Get_GameInstance_Pixels`))) self)
  (`KismetSystemLibrary.K2_ClearAndInvalidateTimerHandle` (`self.Timer_LifeTime`))
  (`/Game/BluePrints/Entities/Monsters/AI/AIC_Monster.Stop_BehaviorTree` (`/Game/Instance/Public/FL_Public.Get_AIC_Monster` self)))

(fn `Monster_KnockBack`
  (params (Attacker :type "Actor Object Reference") (Konckback_Value :type Integer))
  (`MovementComponent.StopMovementImmediately` (`self.CharacterMovement`))
  (`self.LaunchCharacter` (* (`KismetMathLibrary.GetDirectionUnitVector` (`self.K2_GetActorLocation` Attacker) (`self.K2_GetActorLocation`)) (`KismetMathLibrary.Clamp` (- Konckback_Value (`/Game/BluePrints/Entities/Monsters/DataAssets/BP_DA_Monster.Weight` (`self.DataAsset`))) 5 1000)) true) ; 该节点会将MovementMode改为"坠落"
)

(fn `Monster_Setdown_Setting`
  (`CharacterMovementComponent.SetMovementMode` (`self.CharacterMovement`) "MOVE_None" 0)
  (`ActorComponent.SetComponentTickEnabled` (`self.AnimationComponent`) false)
  (`self.SetActorTickEnabled` false)
  (`PrimitiveComponent.SetCollisionResponseToChannel` (`self.CapsuleComponent`) "ECC_Pawn" "ECR_Ignore")
  (`PrimitiveComponent.SetCollisionEnabled` (`self.Sphere_Body`) "NoCollision")
  (`PrimitiveComponent.SetCollisionEnabled` (`self.Box_Weapon`) "NoCollision"))

(fn `Monster_Setup_Data`
  (params (Monster_RowName :type Name))
  (bind _output_get (set `self.Monster_RowName` Monster_RowName))
  (bind _returnvalue (`|GetDataTableRow` "/Game/BluePrints/Entities/Monsters/DT_Monster.DT_Monster" _output_get)
    (:`then`
      (bind ((`Sprite_Flipbook_8_5860318E4FC483DE81F18B9DCD2E083C` _sprite_flipbook) (`AnimSeqence_Rush_22_CC5B2C6E47CCD513EB5FFA9B12F2557D` _animseqence_rush) (`AnimSeqence_Attack_25_12C2D56A419A09278D3ECA8BCE89ACF1` _animseqence_attack) (`DataAsset_11_3A16B7204895299A20C03C8B231E2B82` _dataasset)) (break `/Game/BluePrints/Entities/Monsters/S_Monster` _returnvalue))
      (`PaperFlipbookComponent.SetFlipbook` (`self.Sprite`) _sprite_flipbook)
      (bind _output_get_2 (set `self.DataAsset` _dataasset))
      (set `CharacterMovementComponent.MaxWalkSpeed` (`/Game/BluePrints/Entities/Monsters/DataAssets/BP_DA_Monster.Speed` _output_get_2) (`self.CharacterMovement`))
      (set `self.HP` (`/Game/BluePrints/Entities/Monsters/DataAssets/BP_DA_Monster.HP_Base` _output_get_2))
      (`SceneComponent.SetWorldScale3D` (`self.Sprite`) (`/Game/BluePrints/Entities/Monsters/DataAssets/BP_DA_Monster.Sprite_Size` _output_get_2))
      (`SceneComponent.SetWorldScale3D` (`self.Sphere_Body`) (`/Game/BluePrints/Entities/Monsters/DataAssets/BP_DA_Monster.Collision_Size` _output_get_2))
      (bind _asabp_monster (cast `/Game/BluePrints/Entities/Monsters/ABP_Monster` (`self.GetAnimInstance`)))
      (`/Game/BluePrints/Entities/Monsters/ABP_Monster.Reset` _asabp_monster))))

(fn `Monster_Setup_Setting`
  (`CharacterMovementComponent.SetMovementMode` (`self.CharacterMovement`) "MOVE_Walking" 0)
  (`ActorComponent.SetComponentTickEnabled` (`self.AnimationComponent`) true)
  (`self.SetActorTickEnabled` true)
  (`PrimitiveComponent.SetCollisionResponseToChannel` (`self.CapsuleComponent`) "ECC_Pawn" "ECR_Overlap")
  (`PrimitiveComponent.SetCollisionEnabled` (`self.Sphere_Body`) "QueryOnly")
  (`PrimitiveComponent.SetCollisionEnabled` (`self.Box_Weapon`) "QueryOnly")
  (`KismetSystemLibrary.K2_ClearAndInvalidateTimerHandle` (`self.Timer_AIMove`)))

(fn `Monster_Spawn Damage Number`
  (params (DamageValue :type Integer))
  (bind _returnvalue (`|SpawnActorFromClass` "/Game/UI/BP_UI_DamageNumber.BP_UI_DamageNumber_C" (`KismetMathLibrary.MakeTransform` (`SceneComponent.K2_GetComponentLocation` (`self.Sprite`))) "Undefined" "MultiplyWithRoot" null null))
  (`self.K2_AttachToComponent` _returnvalue (`self.Sprite`) "None" "KeepWorld" "KeepWorld" "KeepWorld" true)
  (`/Game/UI/BP_UI_DamageNumber.Show_DamageNumber` _returnvalue DamageValue))

(fn `Monster_Update_BoxWeaponLocation`
  (bind _box_weapon (`self.Box_Weapon`))
  (bind _direction_x (`KismetMathLibrary.BreakVector2D` (`self.Direction`)))
  (bind _box_weapon_2 (`self.Box_Weapon`))
  (bind _returnvalue (`SceneComponent.GetRelativeTransform` _box_weapon))
  (bind _returnvalue_2 (`SceneComponent.GetRelativeTransform` _box_weapon_2))
  (if (>= _direction_x 0.0)
    (`SceneComponent.K2_SetRelativeLocation` _box_weapon (`KismetMathLibrary.MakeVector` (`KismetMathLibrary.Abs` (.x (.location _returnvalue))) (.y (.location _returnvalue)) (.z (.location _returnvalue))) false false)
    (else
      (`SceneComponent.K2_SetRelativeLocation` _box_weapon_2 (`KismetMathLibrary.MakeVector` (* (`KismetMathLibrary.Abs` (.x (.location _returnvalue_2))) -1.0) (.y (.location _returnvalue_2)) (.z (.location _returnvalue_2))) false false))))

(fn `UserConstructionScript`
  (`self.Monster_Setup_Data` (`self.Monster_RowName`))
  (set `self.Monster_State` "NewEnumerator0") ; 放置在Map中的怪物默认为Awake
)