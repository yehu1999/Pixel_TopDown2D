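; Monster data asset that holds one monster's stats, projectile row and learned skills.
; Init_DataAsset fills every field from a DT_Monster_DA_Init row through a single setter.
; Learned skills live in a tag-to-rank map, where learning a skill adds it at rank 1 or raises its rank.
; Helper functions check a skill's rank and read cycle time and duration from DT_Monster_Skill.
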(fn `Asset Check This Skill`
  (params (Skill_Tag :type Name))
  (returns (Skill_Rank :type Integer) (Has_Learned_ThisSkill :type Boolean))
  (bind (_value _returnvalue) (`BlueprintMapLibrary.Map_Find` (`self.Skills_Learned`) Skill_Tag))
  (return _value _returnvalue))

(fn `Asset_Get_Skill_CycleTime`
  (params (Skill_RowName :type Name))
  (returns (CycleTime :type "Float (double-precision)"))
  (bind _returnvalue (`|GetDataTableRow` "/Game/BluePrints/Entities/Monsters/Skills/DT_Monster_Skill.DT_Monster_Skill" Skill_RowName)
    (:`then`
      (return (`.CycleTime_12_E28FF4DD46CEFE108765E9BB6F01E14F` (break `/Game/BluePrints/Entities/Monsters/Skills/S_Monster_Skill` _returnvalue))))))

(fn `Asset_Get_Skill_Duration`
  (params (Skill_RowName :type Name))
  (returns (Duration :type "Float (double-precision)"))
  (bind _returnvalue (`|GetDataTableRow` "/Game/BluePrints/Entities/Monsters/Skills/DT_Monster_Skill.DT_Monster_Skill" Skill_RowName)
    (:`then`
      (return (`.Duration_14_5C5ED7CF4C5D856962740F82A489BE06` (break `/Game/BluePrints/Entities/Monsters/Skills/S_Monster_Skill` _returnvalue))))))

(fn `Asset_LearnSkill`
  (params (SkillTag :type Name))
  (returns (NewSkillRank :type Integer))
  (locals (Local_NewSkillRank :type Integer))
  (bind _skills_learned (`self.Skills_Learned`))
  (bind (_value _returnvalue) (`BlueprintMapLibrary.Map_Find` _skills_learned SkillTag))
  (if _returnvalue
    (bind _result (`/Engine/EditorBlueprintResources/StandardMacros.IncrementInt` _value)
      (:`  `
        (bind _output_get (set `local.Local_NewSkillRank` _result))
        (`BlueprintMapLibrary.Map_Add` _skills_learned SkillTag _output_get)))
    (else
      (`BlueprintMapLibrary.Map_Add` (`self.Skills_Learned`) SkillTag 1)
      (set `local.Local_NewSkillRank` 1)))
  (return (`local.Local_NewSkillRank`)))

(fn `Asset_Set_All`
  (params (Monster_Name :type Name) (Monster_ID :type Integer) (HP_Base :type Integer) (EXP_Base :type Integer) (Weight :type Integer) (Power :type Integer) (Damage_Value :type Integer) (KnockValue_Value :type Integer) (MultiShoot_Amount :type Integer) (Speed :type "Float (double-precision)") (LifeTime :type "Float (double-precision)") (Sprite_Size :type "Vector Structure") (Collision_Size :type "Vector Structure") (Projectile_RowName :type Name) (Skills_Learned :type "Map of Name to Integer"))
  (set `self.Monster_Name` Monster_Name)
  (set `self.Monster_ID` Monster_ID)
  (set `self.HP_Base` HP_Base)
  (set `self.EXP_Base` EXP_Base)
  (set `self.Weight` Weight)
  (set `self.Power` Power)
  (set `self.Damage_Value` Damage_Value)
  (set `self.KnockValue_Value` KnockValue_Value)
  (set `self.MultiShoot_Amount` MultiShoot_Amount)
  (set `self.Speed` Speed)
  (set `self.LifeTime` LifeTime)
  (set `self.Sprite_Size` Sprite_Size)
  (set `self.Collision_Size` Collision_Size)
  (set `self.Projectile_RowName` Projectile_RowName)
  (set `self.Skills_Learned` Skills_Learned)
  (return))

(fn `Init_DataAsset`
  (params (Monster_RowName :type Name))
  (bind _returnvalue (`|GetDataTableRow` "/Game/BluePrints/Entities/Monsters/DataAssets/DA_Init/DT_Monster_DA_Init.DT_Monster_DA_Init" Monster_RowName)
    (:`then`
      (bind (_monster_name _monster_id _hp_base _exp_base _weight _power _damage_value _knockback_value _multishoot_amount _speed _lifetime _sprite_size _collision_size _projectile_rowname _skills_learned) (break `/Game/BluePrints/Entities/Monsters/DataAssets/DA_Init/S_Monster_DA_Init` _returnvalue))
      (`self.Asset_Set_All` _monster_name _monster_id _hp_base _exp_base _weight _power _damage_value _knockback_value _multishoot_amount _speed _lifetime _sprite_size _collision_size _projectile_rowname _skills_learned)
      (return))))