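; Base NPC Blueprint: a flipbook-sprite character configured from a DT_NPC row and its data assets.
; Construction initializes the data assets, then applies the row's flipbook, stats and component scales and resets ABP_NPC.
; Tick locks actor rotation and keeps the last non-zero XY velocity as Direction for directional animation.
; Interaction overlap stores the Character, Talk updates the dialog widget, and profile loading and skill lookup are stubs.
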(event `self.ReceiveTick`
  (params (DeltaSeconds :type "Float (single-precision)"))
  (bind _returnvalue (`self.GetVelocity`))
  (`self.K2_SetActorRotation` (struct)) ; Keep Actor Rotation
  (if (not (== (`KismetMathLibrary.VSizeXY` _returnvalue) 0.0))
    (set `self.Direction` (`KismetMathLibrary.MakeVector2D` (.x _returnvalue) (.y _returnvalue))) ; ABP将根据Direction改变不同朝向的动画
  ))

(event `self.Box_Interaction.OnComponentBeginOverlap`
  (params (OverlappedComponent :type "PrimitiveComponent Object Reference") (OtherActor :type "Actor Object Reference") (OtherComp :type "PrimitiveComponent Object Reference") (OtherBodyIndex :type Integer) (bFromSweep :type Boolean) (SweepResult :type "HitResult Structure (by ref)"))
  (if (`self.ActorHasTag` OtherActor "Character")
    (bind _asbp_character (cast `/Game/BluePrints/Entities/Characters/BP_Character` OtherActor))
    (set `self.Interacting_Character` _asbp_character)))

(event `/Game/Interfaces/BPI_Dialog.Talk`
  (params (WB_Dialog :type "/Game/UI/Dialog/WB_Dialog Object Reference"))
  (`/Game/UI/Dialog/WB_Dialog.Update_Dialog` WB_Dialog))

(fn `Has Learned This Skill`
  (params (SkillTag :type Name))
  (returns (SkillRank :type Integer) (Has_Learn_ThisSkill :type Boolean))
  (return 0 false))

(fn `NPC_Init_DataAsset`
  (params (Is_From_DT_DA_Init :type Boolean) (Is_From_Profile :type Boolean))
  (if Is_From_DT_DA_Init
    (`/Game/BluePrints/Entities/NPC/DataAsset/BP_DA_NPC.Init_DataAsset` (`self.Data_Asset`) (`self.NPC_RowName`))
    (`/Game/Dialog/DataAsset/BP_DA_Dialog.Init_DataAsset` (`self.Data Asset Dialog`))
    (return)
    (else
      ;[1 1 1] TODO
      (if Is_From_Profile
        _))))

(fn `NPC_Setup_BaseData`
  (params (NPC_RowName :type Name))
  (bind _output_get (set `self.NPC_RowName` NPC_RowName))
  (`self.NPC_Init_DataAsset` true)
  (bind _returnvalue (`|GetDataTableRow` "/Game/BluePrints/Entities/NPC/DT_NPC.DT_NPC" _output_get)
    (:`then`
      (bind ((`Sprite_Flipbook_5_F4D54B7E401AD1B0E1B06ABAB5219E44` _sprite_flipbook) (`DataAsset_7_1DE80DDB4DE93222C456D38599675B7B` _dataasset) (`DataAsset_Dialog_12_D483C344464B389B100D61AAF1F7C53E` _dataasset_dialog)) (break `/Game/BluePrints/Entities/NPC/S_NPC` _returnvalue))
      (`PaperFlipbookComponent.SetFlipbook` (`self.Sprite`) _sprite_flipbook)
      (set `self.Data_Asset` _dataasset)
      (set `self.Data Asset Dialog` _dataasset_dialog)
      (set `CharacterMovementComponent.MaxWalkSpeed` (`/Game/BluePrints/Entities/NPC/DataAsset/BP_DA_NPC.Speed` _dataasset) (`self.CharacterMovement`))
      (set `self.HP` (`/Game/BluePrints/Entities/NPC/DataAsset/BP_DA_NPC.HP Base` _dataasset))
      (`SceneComponent.SetWorldScale3D` (`self.Sprite`) (`/Game/BluePrints/Entities/NPC/DataAsset/BP_DA_NPC.Sprite Size` _dataasset))
      (`SceneComponent.SetWorldScale3D` (`self.Sphere_Body`) (`/Game/BluePrints/Entities/NPC/DataAsset/BP_DA_NPC.Collision Size` _dataasset))
      (`SceneComponent.SetWorldScale3D` (`self.Sphere_ItemMagnet`) (`/Game/BluePrints/Entities/NPC/DataAsset/BP_DA_NPC.Pickup Sphere Size` _dataasset))
      (bind _asabp_npc (cast `/Game/BluePrints/Entities/NPC/ABP_NPC` (`self.GetAnimInstance`)))
      (`/Game/BluePrints/Entities/NPC/ABP_NPC.Reset` _asabp_npc))))

(fn `UserConstructionScript`
  (`self.NPC_Setup_BaseData` (`self.NPC_RowName`)))