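; BP_DA_NPC is an NPC data asset holding name, base HP, speed and size settings for sprite, collision and pickup sphere.
; InitDataAsset looks up a row by name in DT_NPC_Init and, when found, passes its fields to AssetSetAll, which stores them in the asset's variables.
; Only the Row Found branch is wired, so a missing row leaves the values untouched.
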(fn `Asset_Set_All`
  (params (`NPC Name` :type Text) (`HP Base` :type Integer) (Speed :type "Float (double-precision)") (`Sprite Size` :type "Vector Structure") (`Collision Size` :type "Vector Structure") (`Pickup Sphere Size` :type "Vector Structure"))
  (set `self.NPC Name` `NPC Name`)
  (set `self.HP Base` `HP Base`)
  (set `self.Speed` Speed)
  (set `self.Sprite Size` `Sprite Size`)
  (set `self.Collision Size` `Collision Size`)
  (set `self.Pickup Sphere Size` `Pickup Sphere Size`)
  (return))

(fn `Init_DataAsset`
  (params (RowName :type Name))
  (bind _returnvalue (`|GetDataTableRow` "/Game/BluePrints/Entities/NPC/DataAsset/DataAsset_Init/DT_NPC_Init.DT_NPC_Init" RowName)
    (:`then`
      (bind (_npc_name _hp_base _speed _sprite_size _collision_size _pickupsphere_size) (break `/Game/BluePrints/Entities/NPC/DataAsset/DataAsset_Init/S_NPC_Init` _returnvalue))
      (`self.Asset_Set_All` _npc_name _hp_base _speed _sprite_size _collision_size _pickupsphere_size)
      (return))))