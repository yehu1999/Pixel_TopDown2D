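; Character data asset holding stats, size settings, learned and unlocked skills, and row names for projectile, summon and surround entries.
; Init copies a DT_Character_DA_Init row into its variables, with setters for individual stats.
; Level is derived from total EXP by subtracting successive DT_Level thresholds, returning leftover EXP.
; Learning a skill raises its rank in a tag-to-rank map, then prunes skills at DT_Character_Skill max rank from the unlocked list.
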(fn `Assest_Remove_MaxRankSkill_From_Unlocked`
  (for (_array_element _array_index) (`self.Skills_Unlocked`)
    (bind (_value _returnvalue) (`BlueprintMapLibrary.Map_Find` (`self.Skills_Learned`) _array_element))
    (if _returnvalue
      (bind _returnvalue_2 (`|GetDataTableRow` "/Game/BluePrints/Entities/Characters/Skills/DT_Character_Skill.DT_Character_Skill" _array_element)
        (:`then`
          (if (>= _value (`.Max_Rank_23_70FACD7E4C7B63A7778C06A9EA05DA9B` (break `/Game/BluePrints/Entities/Characters/Skills/S_Character_Skill` _returnvalue_2)))
            (`KismetArrayLibrary.Array_Remove` (`self.Skills_Unlocked`) _array_index))))))
  (return))

(fn `Asset Check This Skill`
  (params (Skill_Tag :type Name))
  (returns (Skill_Rank :type Integer) (Has_Learned_ThisSkill :type Boolean))
  (bind (_value _returnvalue) (`BlueprintMapLibrary.Map_Find` (`self.Skills_Learned`) Skill_Tag))
  (return _value _returnvalue))

(fn `Asset_Calculate_Level`
  (params (EXP_All :type Integer))
  (returns (Level :type Integer) (EXP :type Integer) (EXP_Base :type Integer))
  (locals (Local_EXP :type Integer) (Local_Level :type Integer))
  (set `local.Local_EXP` EXP_All)
  (bind _outrownames (`DataTableFunctionLibrary.GetDataTableRowNames` "/Game/BluePrints/Entities/Characters/LevelUp/DT_Level.DT_Level"))
  (for (_array_element _array_index) _outrownames
    (bind _returnvalue (`|GetDataTableRow` "/Game/BluePrints/Entities/Characters/LevelUp/DT_Level.DT_Level" _array_element)
      (:`then`
        (bind _exp_base (break `/Game/BluePrints/Entities/Characters/LevelUp/S_Level` _returnvalue))
        (bind _returnvalue_2 (- (`local.Local_EXP`) _exp_base))
        (if (< _returnvalue_2 0)
          (break)
          (else
            (set `local.Local_EXP` _returnvalue_2))))))
  (set `local.Local_Level` _array_index)
  (set `self.EXP_Base` _exp_base)
  (return (`local.Local_Level`) (`local.Local_EXP`) (`self.EXP_Base`)))

(fn `Asset_DEBUG_Print_Skill`
  (bind _skills_learned (`self.Skills_Learned`))
  (bind _keys (`BlueprintMapLibrary.Map_Keys` _skills_learned))
  (bind _values (`BlueprintMapLibrary.Map_Values` _skills_learned))
  (for (_array_element _array_index) _keys
    (`KismetSystemLibrary.PrintText` null (`|FormatText` "Skill{Index}: {Tag} Rank {NUM}" _array_index _array_element (`|GetArrayItem` _values _array_index)))))

(fn `Asset_LearnSkill`
  (params (SkillTag :type Name))
  (returns (NewSkillRank :type Integer))
  (locals (Local_NewSkillRank :type Integer))
  (bind _skills_learned (`self.Skills_Learned`))
  (bind (_value _returnvalue) (`BlueprintMapLibrary.Map_Find` _skills_learned SkillTag))
  (if _returnvalue
    (bind _result (`/Engine/EditorBlueprintResources/StandardMacros.IncrementInt` _value)
      (:`  `
        (bind _output_get (set `local.Local_NewSkillRank` _result))
        (`BlueprintMapLibrary.Map_Add` _skills_learned SkillTag _output_get)))
    (else
      (`BlueprintMapLibrary.Map_Add` (`self.Skills_Learned`) SkillTag 1)
      (set `local.Local_NewSkillRank` 1)))
  (`self.Assest_Remove_MaxRankSkill_From_Unlocked`)
  (return (`local.Local_NewSkillRank`)))

(fn `Asset_Set_All`
  (params (Character_Name :type Text) (HP_Base :type Integer) (EXP_Base :type Integer) (Weight :type Integer) (Power :type Integer) (Magic_Power :type Integer) (MultiShoot_Amount :type Integer) (Speed :type "Float (double-precision)") (Sprite_Size :type "Vector Structure") (Collision_Size :type "Vector Structure") (PickupSphere_Size :type "Vector Structure") (Skills_Unlocked :type "Array of Name") (Skills_Learned :type "Map of Name to Integer") (Projectile_RowName :type Name) (Summon_RowName :type Name) (Surround_RowName :type Name))
  (set `self.Character_Name` Character_Name)
  (set `self.HP_Base` HP_Base)
  (set `self.EXP_Base` EXP_Base)
  (set `self.Weight` Weight)
  (set `self.Power` Power)
  (set `self.Magic_Power` Magic_Power)
  (set `self.MultiShoot_Amount` MultiShoot_Amount)
  (set `self.Speed` Speed)
  (set `self.Sprite_Size` Sprite_Size)
  (set `self.Collision_Size` Collision_Size)
  (set `self.PickupSphere_Size` PickupSphere_Size)
  (set `self.Skills_Unlocked` Skills_Unlocked)
  (set `self.Skills_Learned` Skills_Learned)
  (set `self.Projectile_RowName` Projectile_RowName)
  (set `self.Summon_RowName` Summon_RowName)
  (set `self.Surround_RowName` Surround_RowName))

(fn `Asset_Set_MultiShoot_Amount`
  (params (MultiShoot_Amount :type Integer))
  (set `self.MultiShoot_Amount` MultiShoot_Amount))

(fn `Asset_Set_PickupSphere_Size`
  (params (PickupSphere_Size :type "Vector Structure"))
  (set `self.PickupSphere_Size` PickupSphere_Size))

(fn `Asset_Set_Power`
  (params (Power :type Integer))
  (set `self.Power` Power))

(fn `Asset_Set_SetHP_Base`
  (params (New_HP_Base :type Integer))
  (set `self.HP_Base` New_HP_Base))

(fn `Asset_Set_Speed_Base`
  (params (New_Speed_Base :type "Float (double-precision)"))
  (set `self.Speed` New_Speed_Base))

(fn `Init_DataAsset`
  (params (Character_RowName :type Name))
  (bind _returnvalue (`|GetDataTableRow` "/Game/BluePrints/Entities/Characters/DataAssets/Init_DA/DT_Character_DA_Init.DT_Character_DA_Init" Character_RowName)
    (:`then`
      (bind (_character_name _hp_base _exp_base _weight _power _magic_power _multishoot_amount _speed _sprite_size _collision_size _pickupsphere_size _skills_unlocked _skills_learned _projectile_rowname _summon_rowname _surround_rowname) (break `/Game/BluePrints/Entities/Characters/DataAssets/Init_DA/S_Character_DA_Init` _returnvalue))
      (`self.Asset_Set_All` _character_name _hp_base _exp_base _weight _power _magic_power _multishoot_amount _speed _sprite_size _collision_size _pickupsphere_size _skills_unlocked _skills_learned _projectile_rowname _summon_rowname _surround_rowname)
      (`self.Assest_Remove_MaxRankSkill_From_Unlocked`)
      (return))))