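; Backpack component that holds a fixed-size slot inventory for the player or an NPC.
; Adding stacks items by row name or fills the first empty slot, while removal can spawn drops through the actor pool.
; Changes are pushed to backpack widgets, or to the trade widget for NPC removals.
; For players it also creates the UI, adds test starter items and sphere-traces every tick to show nearby-object hints.
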(event `Init_Backpack`
  (for _ (range (`self.Backpack_MaxSize`))
    (`KismetArrayLibrary.Array_Add` (`self.Backpack_Inventory`) (`self.Backpack_EmptySlot`))))

(event `self.ReceiveBeginPlay`
  (`self.Init_Backpack`)
  (if (not (`self.Is_NPC`))
    (`self.UI_Init`)
    (`self.TEST_AddSomeObject`)))

(event `self.ReceiveTick`
  (params (DeltaSeconds :type "Float (single-precision)"))
  (bind _returnvalue (`Actor.K2_GetActorLocation` (`self.Owner_Pawn`)))
  (if (not (`self.Is_NPC`))
    (bind (_outhits _returnvalue_2) (`KismetSystemLibrary.SphereTraceMultiForObjects` :`Start` _returnvalue :`End` _returnvalue :`Radius` 20.0 :`ObjectTypes` (`|MakeArray` "ObjectTypeQuery9" "ObjectTypeQuery7" :!type "EObjectTypeQuery Enum") :`DrawDebugType` "ForOneFrame")) ; HintText很愚钝的实现方法
    (if _returnvalue_2
      (for _array_element _outhits
        (bind (_object_type _object_rowname) (message `/Game/Interfaces/BPI_Object.Get_Object_Info` (`.HitActor` (`GameplayStatics.BreakHitResult` _array_element))))
        (`/Game/UI/Backpack/WB_Backpack_HintBox.Show_HintBox` (`self.WB_HintBox`) true _object_type _object_rowname))
      (else
        (`/Game/UI/Backpack/WB_Backpack_HintBox.Show_HintBox` (`self.WB_HintBox`) false "NewEnumerator6" "None")))))

(fn `Add_Object_ToInventory`
  (params (S_InventoryContent :type "/Game/BluePrints/Objects/S_InventoryContent Structure (by ref)"))
  (returns (Is_Successed :type Boolean))
  (locals (Local_Is_ObjectFound :type Boolean) (Local_Content_ToAdd :type "/Game/BluePrints/Objects/S_InventoryContent Structure") (Local_New_InventoryContent :type "/Game/BluePrints/Objects/S_InventoryContent Structure") (Local_Added_InventoryIndex :type Integer))
  (bind _backpack_inventory (`self.Backpack_Inventory`))
  (bind (_object_type _object_rowname _object_amount) (break `/Game/BluePrints/Objects/S_InventoryContent` (`local.Local_Content_ToAdd`)))
  (bind _returnvalue (`KismetArrayLibrary.Array_Find` _backpack_inventory (`self.Backpack_EmptySlot`)))
  (bind _output_get (set `local.Local_Content_ToAdd` S_InventoryContent))
  (set `local.Local_New_InventoryContent` _output_get)
  (bind (_object_sprite _object_icon _maxamount_inventorycontent _object_name _object_description _is_allowed_addtoinventory) (`/Game/Instance/Public/FL_Public.Break_Object` _object_type _object_rowname))
  (if _is_allowed_addtoinventory
    (if (> _maxamount_inventorycontent 0)
      (set `local.Local_Is_ObjectFound` false)
      (for (_array_element _array_index) (`self.Backpack_Inventory`)
        (bind (_object_type_2 _object_rowname_2 _object_amount_2) (break `/Game/BluePrints/Objects/S_InventoryContent` _array_element))
        (if (== _object_rowname_2 _object_rowname)
          (bind _structout (setmembers `/Game/BluePrints/Objects/S_InventoryContent` :`StructRef` (`|GetArrayItem` (`self.Backpack_Inventory`) _array_index) :`Object_Amount` (+ _object_amount_2 _object_amount)))
          (set `local.Local_New_InventoryContent` _structout)
          (set `local.Local_Is_ObjectFound` true)
          (set `local.Local_Added_InventoryIndex` _array_index)
          (break)))
      (if (`local.Local_Is_ObjectFound`)
        _
        (elif (>= _returnvalue 0)
          (set `local.Local_Added_InventoryIndex` _returnvalue) ; 先设置Index，后设置背包内容\n不然find函数会在新内容中寻找Empty
          (`|VariableSetRef` (`|GetArrayItem` _backpack_inventory _returnvalue) (`local.Local_Content_ToAdd`))
          (else
            (`/Game/Instance/Public/FL_Public.DEBUG_MYLOG` "NewEnumerator3" "Backpack Is Full, Add Object Failed" "BP_AC_Backpack" "Add Object To Inventory")
            (return false))))
      (`self.UI_Update_InventorySlot` (`local.Local_Added_InventoryIndex`) (`local.Local_New_InventoryContent`))
      (return true))))

(fn `Change Inventory Content`
  (params (Inventory_Index :type Integer) (Object_RowName :type Name))
  (if (>= Inventory_Index 0)
    (bind _structout (setmembers `/Game/BluePrints/Objects/S_InventoryContent` :`StructRef` (`|GetArrayItem` (`self.Backpack_Inventory`) Inventory_Index) :`Object_RowName` Object_RowName))
    (`self.UI_Update_InventorySlot` Inventory_Index _structout)))

(fn `Drop_InventoryContent`
  (params (S_Inventory_Content :type "/Game/BluePrints/Objects/S_InventoryContent Structure"))
  (bind (_object_type _object_rowname _object_amount) (break `/Game/BluePrints/Objects/S_InventoryContent` S_Inventory_Content))
  (`/Game/Instance/Public/FL_Public.DEBUG_MYLOG` "NewEnumerator0" (`|FormatText` "Drop {A}*{B}" _object_rowname _object_amount))
  (`/Game/Instance/BP_ActorPool.Awake_Num_Object` (`/Game/Instance/Public/FL_Public.Get_ActorPool`) _object_type _object_rowname _object_amount (`Actor.K2_GetActorLocation` (`/Game/Instance/Public/FL_Public.Get_Character`)) 10.0)
  (return))

(fn `Remove_Object_FromInventory`
  (params (Inventory_Index :type Integer) (Remove_Amount :type Integer) (Is_Spawn_DropObject :type Boolean))
  (returns (Is_Successed :type Boolean) (Is_Empty :type Boolean))
  (locals (Local_Content_ToDrop :type "/Game/BluePrints/Objects/S_InventoryContent Structure") (Local_NewInventoryContent :type "/Game/BluePrints/Objects/S_InventoryContent Structure") (Local_IsEmpty :type Boolean))
  (bind _output (`|GetArrayItem` (`self.Backpack_Inventory`) Inventory_Index))
  (bind (_object_type _object_rowname _object_amount) (break `/Game/BluePrints/Objects/S_InventoryContent` _output))
  (bind _returnvalue (- _object_amount Remove_Amount))
  (if (> Remove_Amount 0)
    (if (`|EnumInequality` _object_type "NewEnumerator6")
      (set `local.Local_Content_ToDrop` (make `/Game/BluePrints/Objects/S_InventoryContent` _object_type _object_rowname _object_amount))
      (if (<= _returnvalue 0)
        (`|VariableSetRef` _output (`self.Backpack_EmptySlot`))
        (set `local.Local_NewInventoryContent` (`self.Backpack_EmptySlot`))
        (set `local.Local_IsEmpty` true)
        (else
          (bind _structout (setmembers `/Game/BluePrints/Objects/S_InventoryContent` :`StructRef` _output :`Object_Amount` _returnvalue))
          (setmembers `/Game/BluePrints/Objects/S_InventoryContent` :`StructRef` (`local.Local_Content_ToDrop`) :`Object_Amount` Remove_Amount)
          (set `local.Local_NewInventoryContent` _structout)
          (set `local.Local_IsEmpty` false)))
      (if (`self.Is_NPC`)
        (`self.UI_Update_TradeSlot`)
        (else
          (`self.UI_Update_InventorySlot` Inventory_Index (`local.Local_NewInventoryContent`))))
      (if Is_Spawn_DropObject
        (`self.Drop_InventoryContent` (`local.Local_Content_ToDrop`)))
      (return true (`local.Local_IsEmpty`))
      (else
        (return false false)))))

(fn `Switch_InventorySlot`
  (params (Inventory_Index1 :type Integer) (Inventory_Index2 :type Integer))
  (bind _backpack_maxsize (`self.Backpack_MaxSize`))
  (`|ExecutionSequence`
    (:`then_0`
      (if (and (`KismetMathLibrary.InRange_IntInt` Inventory_Index1 0 _backpack_maxsize true false) (`KismetMathLibrary.InRange_IntInt` Inventory_Index2 0 _backpack_maxsize true false))
        (`KismetArrayLibrary.Array_Swap` (`self.Backpack_Inventory`) Inventory_Index1 Inventory_Index2)
        (else
          (`/Game/Instance/Public/FL_Public.DEBUG_MYLOG` "NewEnumerator2" "Switching Index Is Invalid" "BP_AC_Backpack" "Switch_InventorySlot"))))
    (:`then_1`
      (`self.UI_Update_InventorySlot` Inventory_Index1 (`|GetArrayItem` (`self.Backpack_Inventory`) Inventory_Index1))
      (`self.UI_Update_InventorySlot` Inventory_Index2 (`|GetArrayItem` (`self.Backpack_Inventory`) Inventory_Index2))
      (return))))

(fn `TEST_AddSomeObject`
  (`self.Add_Object_ToInventory` (make `/Game/BluePrints/Objects/S_InventoryContent` "NewEnumerator5" "Tool_Spade" 1))
  (`self.Add_Object_ToInventory` (make `/Game/BluePrints/Objects/S_InventoryContent` "NewEnumerator5" "Tool_Bucket_Empty" 1))
  (`self.Add_Object_ToInventory` (make `/Game/BluePrints/Objects/S_InventoryContent` "NewEnumerator5" "Tool_Sickle" 1))
  (`self.Add_Object_ToInventory` (make `/Game/BluePrints/Objects/S_InventoryContent` "NewEnumerator7" "Seed_Rose" 8))
  (`self.Add_Object_ToInventory` (make `/Game/BluePrints/Objects/S_InventoryContent` "NewEnumerator7" "Seed_Turnip" 8)))

(fn `UI_Init`
  (bind _owner_controller (`self.Owner_Controller`))
  (`|ExecutionSequence`
    (:`then_0`
      (bind _aspawn (cast `Pawn` (`self.GetOwner`)))
      (bind _output_get (set `self.Owner_Pawn` _aspawn))
      (bind `_as玩家控制器` (cast `PlayerController` (`Pawn.GetController` _output_get)))
      (set `self.Owner_Controller` `_as玩家控制器`))
    (:`then_1`
      (bind _returnvalue (`|CreateWidget` "/Game/UI/Backpack/WB_Backpack_HintBox.WB_Backpack_HintBox_C" _owner_controller))
      (bind _output_get_2 (set `self.WB_HintBox` _returnvalue))
      (`UserWidget.AddToViewport` _output_get_2 0))
    (:`then_2`
      (bind _returnvalue_2 (`|CreateWidget` "/Game/UI/Backpack/WB_Backpack.WB_Backpack_C" _owner_controller))
      (bind _output_get_3 (set `self.WB_Backpack` _returnvalue_2))
      (`UserWidget.AddToViewport` _output_get_3 1) ; ZOrder=1
    )
    (:`then_3`
      (bind _returnvalue_3 (`|CreateWidget` "/Game/UI/Backpack/WB_DropPanel.WB_DropPanel_C" _owner_controller))
      (bind _output_get_4 (set `self.WB_DropPanel` _returnvalue_3))
      (`UserWidget.AddToViewport` _output_get_4 1) ; ZOrder=1
    )))

(fn `UI_Init_BuyPanel`
  (params (BP_NPC :type "/Game/BluePrints/Entities/NPC/BP_NPC Object Reference"))
  (bind _wb_buypanel (`self.WB_BuyPanel`))
  (`/Engine/EditorBlueprintResources/StandardMacros.IsValid` _wb_buypanel
    (:`Is Valid`
      (set `/Game/UI/Trade/WB_BuyPanel.BP_NPC` BP_NPC _wb_buypanel))
    (:`Is Not Valid`
      (bind _returnvalue (`|CreateWidget` "/Game/UI/Trade/WB_BuyPanel.WB_BuyPanel_C" (`self.Owner_Controller`) BP_NPC))
      (bind _output_get (set `self.WB_BuyPanel` _returnvalue))
      (`UserWidget.AddToViewport` _output_get 1) ; ZOrder=1
    )))

(fn `UI_Update_InventorySlot`
  (params (Inventory_Index :type Integer) (New_S_InventoryContent :type "/Game/BluePrints/Objects/S_InventoryContent Structure"))
  (`/Game/UI/Backpack/WB_Backpack.Update_Backpack_Slot` (`self.WB_Backpack`) Inventory_Index New_S_InventoryContent))

(fn `UI_Update_TradeSlot`
  (`/Game/UI/Trade/WB_Trade.Update_Trade` (`/Game/BluePrints/Entities/Characters/BP_Character.WB_Trade` (`/Game/Instance/Public/FL_Public.Get_Character`))))